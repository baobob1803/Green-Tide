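; Wave manager for a room that spawns timed waves of orcs and flags the room completed once all are dead.
; BeginPlay collects tagged TargetPoints, then GenerateWave scales enemy count by room level and staggers spawns at random points, with the WavesTempo macro pacing waves.
; Orcs receive the level and a manager reference; DestroyUnite removes them from the tracked list, calls the player's RewardExp and destroys them, while a delay loop polls for an empty list.
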(event `DestroyUnite`
  (params (`Dead Unit` :type "/Game/ProjectContent/Enemies/BP_Enemy Object Reference (by ref)"))
  (`KismetArrayLibrary.Array_RemoveItem` (`self.listOfSpawnedEnemies`) `Dead Unit`)
  (`/Game/ThirdPersonBP/Blueprints/BP_Character_Master.RewardExp` (`self.player`) 0.0)
  (`self.K2_DestroyActor` `Dead Unit`))

(event `self.ReceiveBeginPlay`
  (set `self.roomCompleted` false)
  (bind _outactors (`GameplayStatics.GetAllActorsOfClassWithTag` "/Script/Engine.TargetPoint" "SpawnPoints"))
  (set `self.listOfSpawnPoints` _outactors)
  (`KismetSystemLibrary.PrintString` "InitSpawnPoints")
  (`KismetSystemLibrary.Delay` 5.0)
  (`self.GenerateWave` 60))

(event `GenerateWave`
  (params (CurrentRoomLevel :type Integer))
  (set `self.tempEnemiesIndex` 0)
  (bind _output_get (set `self.currentRoomLevel` CurrentRoomLevel))
  (`/Engine/EditorBlueprintResources/StandardMacros.CompareInt` _output_get 50
    (:`>`
      (`/Engine/EditorBlueprintResources/StandardMacros.CompareInt` _output_get 100
        (:`>`
          (set `self.nbOfEnemiesToSpawn` 7))
        (:`==`
          (set `self.nbOfEnemiesToSpawn` 5 :!label _label))
        (:`<`
          (goto _label))))
    (:`==`
      (set `self.nbOfEnemiesToSpawn` 3 :!label _label_2))
    (:`<`
      (goto _label_2)))
  (bind _output_get_2 (set `self.nbOfWaves` 3))
  (set `self.timeBetweenWaves` 15.0)
  (`/Engine/EditorBlueprintResources/StandardMacros.CompareInt` _output_get_2 :!label _label_3
    (:`>`
      (if (== (`self.nbOfEnemiesToSpawn`) (`self.tempEnemiesIndex`))
        (`self.WavesTempo` (`self.nbOfWaves`)
          (:`Completed`
            (goto _label_3)))
        (else
          (`KismetSystemLibrary.Delay` 0.4)
          (bind _returnvalue (`|SpawnActorFromClass` "/Game/ProjectContent/Enemies/BP_Orc.BP_Orc_C" (`self.GetTransform` (`KismetArrayLibrary.Array_Random` (`self.listOfSpawnPoints`))) "AdjustIfPossibleButAlwaysSpawn" "OverrideRootScale" null null))
          (set `/Game/ProjectContent/Enemies/BP_Enemy.waveManager` self _returnvalue)
          (`KismetArrayLibrary.Array_Add` (`self.listOfSpawnedEnemies`) _returnvalue)
          (set `/Game/ProjectContent/Enemies/BP_Enemy.enemyLevel` (`self.currentRoomLevel`) _returnvalue)
          (`/Engine/EditorBlueprintResources/StandardMacros.IncrementInt` (`self.tempEnemiesIndex`)
            (:`  `
              (goto _label_3))))))
    (:`==`
      (`KismetSystemLibrary.PrintString` "No more wave")
      (`KismetSystemLibrary.Delay` 2.0 :!label _label_4)
      (`/Engine/EditorBlueprintResources/StandardMacros.CompareInt` (`KismetArrayLibrary.Array_Length` (`self.listOfSpawnedEnemies`))
        (:`>`
          (goto _label_4))
        (:`==`
          (set `self.roomCompleted` true)
          (`KismetSystemLibrary.PrintString` "RoomCompleted"))))))

(fn `UserConstructionScript`)