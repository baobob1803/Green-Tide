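; BP_Enemy is an enemy that tracks its own health and is removed through a wave manager when killed.
; AnyDamage subtracts the truncated damage from HealthPoint and prints the remaining value as debug output.
; At zero health or below, it passes itself to WaveManager's DestroyUnite instead of destroying itself directly.
; BeginPlay, overlap, Tick and the construction script are empty.
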(event `self.ReceiveAnyDamage`
  (params (Damage :type "Float (single-precision)") (DamageType :type "DamageType Object Reference") (InstigatedBy :type "Controller Object Reference") (DamageCauser :type "Actor Object Reference"))
  (bind _healthpoint (`self.healthPoint`))
  (bind _output_get (set `self.healthPoint` (- _healthpoint (`KismetMathLibrary.FTrunc` Damage))))
  (`KismetSystemLibrary.PrintString` (`KismetStringLibrary.Conv_IntToString` _output_get))
  (if (<= _healthpoint 0)
    (`/Game/ProjectContent/Enemies/BP_WaveManager.DestroyUnite` (`self.waveManager`) self)))

(fn `UserConstructionScript`)