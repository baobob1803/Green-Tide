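; BP_LevelManager runs the main menu: it opens the main, profile and profile-creation widgets and handles player profile creation.
; On BeginPlay it caches BP_GameInstance, copies its profile array locally and shows the main menu.
; Confirming creation rejects empty names, duplicates and a full list, then spawns a BP_PlayerProfile actor with name and ID.
; The updated array is written back to the game instance and the creation widget closes.
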(event `self.ReceiveBeginPlay`
  ;[0.75 0.2602 1] OnBeginPlay Initialization Phase
  ;;[0.4742 0.5065 1] Update the list of profile from the game instance to the local list of profile (On Event start)
  (bind _asbp_game_instance (cast `/Game/ProjectContent/Blueprints/MenuPrincipal/MainMenu/BP_GameInstance` (`GameplayStatics.GetGameInstance`))
    (:`then`
      (bind _output_get (set `self.GameInstanceReference` _asbp_game_instance))
      (set `self.LocalArrayOfPlayerProfiles` (`/Game/ProjectContent/Blueprints/MenuPrincipal/MainMenu/BP_GameInstance.ArrayOfPlayerProfile` _output_get))
      ;;[0.2705 0.88 1] Creating and referencing Main Menu Widget
      (bind _returnvalue (`|CreateWidget` "/Game/ProjectContent/Blueprints/MenuPrincipal/MainMenu/UI_MainMenu_BP.UI_MainMenu_BP_C" (`GameplayStatics.GetPlayerController` 0)))
      (bind _output_get_2 (set `self.MainMenuReference` _returnvalue))
      (`UserWidget.AddToViewport` _output_get_2 0))
    (:`CastFailed`
      (`KismetSystemLibrary.PrintString` "Hello"))))

(event `BackButtonClicked(ProfileMenu)`
  ;[1 0.7581 0.1451 1 36] Profile Menu Linked Events
  ;;[0.4167 0.3531 0.1156] Back From Profile Menu
  (`Widget.RemoveFromParent` (`self.ProfileMenuReference`)))

(event `ProfileMenuButtonClicked`
  ;[1 0.7581 0.1451 1 36] Profile Menu Linked Events
  ;;[0.151 0.1425 0.05282] Profile Button Click
  (bind _returnvalue (`|CreateWidget` "/Game/ProjectContent/Blueprints/MenuPrincipal/MainMenu/CreateProfileMenu/UI_ProfileMenu.UI_ProfileMenu_C" (`GameplayStatics.GetPlayerController` 0)))
  (bind _output_get (set `self.ProfileMenuReference` _returnvalue))
  (`UserWidget.AddToViewport` _output_get 0))

(event `CreateNewProfileButtonTapped`
  ;[1 0.7581 0.1451 1 36] Profile Menu Linked Events
  ;;[1 1 1] Comment
  (bind _returnvalue (`|CreateWidget` "/Game/ProjectContent/Blueprints/MenuPrincipal/MainMenu/CreateProfileMenu/UI_CreateNewProfileMenu.UI_CreateNewProfileMenu_C" (`GameplayStatics.GetPlayerController` 0)))
  (bind _output_get (set `self.CreateNewProfileMenuReference` _returnvalue))
  (`UserWidget.AddToViewport` _output_get 0))

(event `ConfirmProfileCreationClicked`
  (bind _localarrayofplayerprofiles (`self.LocalArrayOfPlayerProfiles`))
  ;[1 1 1] Check + Spawn/Reference Profile
  ;;[1 1 1] Is Submitted Profile Name Empty ?
  (if (`KismetTextLibrary.TextIsEmpty` (`KismetTextLibrary.Conv_StringToText` (`/Game/ProjectContent/Blueprints/MenuPrincipal/MainMenu/CreateProfileMenu/UI_CreateNewProfileMenu.CurrentProfileName` (`self.CreateNewProfileMenuReference`))))
    (`KismetSystemLibrary.PrintString` "Cannot Submit an empty name")
    (`KismetSystemLibrary.CollectGarbage`)
    (else
      ;;[1 1 1] Profile List Full - Check
      (if (== (`KismetArrayLibrary.Array_Length` (`self.LocalArrayOfPlayerProfiles`)) 5)
        (`KismetSystemLibrary.PrintString` "Cannot create more than 5 profiles")
        (`KismetSystemLibrary.CollectGarbage`)
        (else
          ;;[1 1 1] ProfileNameAlreadyExists - Check
          (for _array_element (`self.LocalArrayOfPlayerProfiles`)
            (if (`KismetStringLibrary.EqualEqual_StrStr` (`/Game/ProjectContent/Blueprints/MenuPrincipal/Entities/BP_PlayerProfile.ProfileName` _array_element) (`/Game/ProjectContent/Blueprints/MenuPrincipal/MainMenu/CreateProfileMenu/UI_CreateNewProfileMenu.CurrentProfileName` (`self.CreateNewProfileMenuReference`)))
              (`KismetSystemLibrary.PrintString` "A profile with thime name already exists")
              (set `self.SameNameFound` true)))
          (if (`self.SameNameFound`)
            (`KismetSystemLibrary.PrintString` "Profile Did not spawn")
            (`KismetSystemLibrary.CollectGarbage`)
            (else
              ;;[1 1 1] GeneratingNewProfile and setting arrays
              (bind _returnvalue (`|SpawnActorFromClass` "/Game/ProjectContent/Blueprints/MenuPrincipal/Entities/BP_PlayerProfile.BP_PlayerProfile_C" (`self.Spawn Transform`) "AdjustIfPossibleButAlwaysSpawn" "OverrideRootScale" null null))
              (bind _output_get (set `self.LastCreatedPlayerProfile` _returnvalue))
              (set `/Game/ProjectContent/Blueprints/MenuPrincipal/Entities/BP_PlayerProfile.ProfileName` (`/Game/ProjectContent/Blueprints/MenuPrincipal/MainMenu/CreateProfileMenu/UI_CreateNewProfileMenu.CurrentProfileName` (`self.CreateNewProfileMenuReference`)) _output_get)
              (set `/Game/ProjectContent/Blueprints/MenuPrincipal/Entities/BP_PlayerProfile.profileId` (+ (`KismetArrayLibrary.Array_Length` (`self.LocalArrayOfPlayerProfiles`)) 1) _output_get)
              (`KismetArrayLibrary.Array_Add` _localarrayofplayerprofiles (`self.LastCreatedPlayerProfile`))
              (set `/Game/ProjectContent/Blueprints/MenuPrincipal/MainMenu/BP_GameInstance.ArrayOfPlayerProfile` _localarrayofplayerprofiles (`self.GameInstanceReference`))
              (`Widget.RemoveFromParent` (`self.CreateNewProfileMenuReference`))
              (`KismetSystemLibrary.CollectGarbage`))))))))

(fn `UserConstructionScript`)