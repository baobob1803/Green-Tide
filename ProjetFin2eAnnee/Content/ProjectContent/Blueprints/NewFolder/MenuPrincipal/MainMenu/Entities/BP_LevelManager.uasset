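; Main menu level manager actor that creates the menu widgets and handles player profile creation.
; BeginPlay caches the GameInstance and shows the main menu; button events open the profile and profile-creation widgets or close the profile menu.
; Confirming creation rejects empty names, a full list or duplicate names.
; A valid name spawns a profile actor with a name and index-based ID, then writes the local profile array to the GameInstance.
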(event `self.ReceiveBeginPlay`
  ;[1 1 1] Comment
  (bind _asbp_game_instance (cast `` (`GameplayStatics.GetGameInstance`)))
  (bind (_output_get _output_get_2) (set `self.GameInstanceReference` null _asbp_game_instance))
  (set `self.LocalArrayOfPlayerProfiles` _ (`/Game/ProjectContent/Blueprints/NewFolder/MenuPrincipal/MainMenu/Entities/BP_LevelManager.ArrayOfPlayerProfile` _output_get_2))
  ;[1 1 1] Creating and referencing Main Menu Widget
  (bind _returnvalue (`|CreateWidget` null (`GameplayStatics.GetPlayerController` 0)))
  (bind (_output_get_3 _output_get_4) (set `self.MainMenuReference` null _returnvalue))
  (`UserWidget.AddToViewport` _output_get_4 0))

(event `BackButtonClicked(ProfileMenu)`
  ;[1 0.7581 0.1451 1 36] Profile Menu Linked Events
  ;;[0.4167 0.3531 0.1156] Back From Profile Menu
  (`Widget.RemoveFromParent` (`.ProfileMenuReference` (`self.ProfileMenuReference`))))

(event `ProfileMenuButtonClicked`
  ;[1 0.7581 0.1451 1 36] Profile Menu Linked Events
  ;;[0.151 0.1425 0.05282] Profile Button Click
  (bind _returnvalue (`|CreateWidget` null (`GameplayStatics.GetPlayerController` 0)))
  (bind (_output_get _output_get_2) (set `self.ProfileMenuReference` null _returnvalue))
  (`UserWidget.AddToViewport` _output_get_2 0))

(event `CreateNewProfileButtonTapped`
  ;[1 0.7581 0.1451 1 36] Profile Menu Linked Events
  ;;[1 1 1] Comment
  (bind _returnvalue (`|CreateWidget` null (`GameplayStatics.GetPlayerController` 0)))
  (bind (_output_get _output_get_2) (set `self.CreateNewProfileMenuReference` null _returnvalue))
  (`UserWidget.AddToViewport` _output_get_2 0))

(event `ConfirmProfileCreationClicked`
  (bind (_localarrayofplayerprofiles _localarrayofplayerprofiles_2) (`self.LocalArrayOfPlayerProfiles`))
  (bind (_lastcreatedplayerprofile _lastcreatedplayerprofile_2) (`self.LastCreatedPlayerProfile`))
  ;[1 1 1] Comment
  (if (`KismetTextLibrary.TextIsEmpty` (`KismetTextLibrary.Conv_StringToText` (`/Game/ProjectContent/Blueprints/NewFolder/MenuPrincipal/MainMenu/Entities/BP_LevelManager.CurrentProfileName` (`.CreateNewProfileMenuReference` (`self.CreateNewProfileMenuReference`)))))
    (`KismetSystemLibrary.PrintString` "Cannot Submit an empty name")
    (`KismetSystemLibrary.CollectGarbage`)
    (else
      ;;[1 1 1] Profile List Full - Check
      (if (== (`KismetArrayLibrary.Array_Length` (`.LocalArrayOfPlayerProfiles` (`self.LocalArrayOfPlayerProfiles`))) 5)
        (`KismetSystemLibrary.PrintString` "Cannot create more than 5 profiles")
        (`KismetSystemLibrary.CollectGarbage`)
        (else
          ;;[1 1 1] ProfileNameAlreadyExists - Check
          (for _array_element (`.LocalArrayOfPlayerProfiles` (`self.LocalArrayOfPlayerProfiles`))
            (if (`KismetStringLibrary.EqualEqual_StrStr` (`/Game/ProjectContent/Blueprints/NewFolder/MenuPrincipal/MainMenu/Entities/BP_LevelManager.ProfileName` _array_element) (`/Game/ProjectContent/Blueprints/NewFolder/MenuPrincipal/MainMenu/Entities/BP_LevelManager.CurrentProfileName` (`.CreateNewProfileMenuReference` (`self.CreateNewProfileMenuReference`))))
              (`KismetSystemLibrary.PrintString` "A profile with thime name already exists")
              (set `self.SameNameFound` true)))
          (if (`self.SameNameFound`)
            (`KismetSystemLibrary.PrintString` "Profile Did not spawn")
            (`KismetSystemLibrary.CollectGarbage`)
            (else
              ;;[1 1 1] GeneratingNewProfile and setting arrays
              (bind _returnvalue (`|SpawnActorFromClass` null (`self.Spawn Transform`) "AdjustIfPossibleButAlwaysSpawn" "OverrideRootScale" null null))
              (bind (_output_get _output_get_2) (set `self.LastCreatedPlayerProfile` null _returnvalue))
              (set `/Game/ProjectContent/Blueprints/NewFolder/MenuPrincipal/MainMenu/Entities/BP_LevelManager.ProfileName` (`/Game/ProjectContent/Blueprints/NewFolder/MenuPrincipal/MainMenu/Entities/BP_LevelManager.CurrentProfileName` (`.CreateNewProfileMenuReference` (`self.CreateNewProfileMenuReference`))) _output_get_2)
              (bind _returnvalue_2 (`KismetArrayLibrary.Array_Add` _localarrayofplayerprofiles_2 _lastcreatedplayerprofile_2))
              (set `/Game/ProjectContent/Blueprints/NewFolder/MenuPrincipal/MainMenu/Entities/BP_LevelManager.profileId` _returnvalue_2 _lastcreatedplayerprofile_2)
              (set `/Game/ProjectContent/Blueprints/NewFolder/MenuPrincipal/MainMenu/Entities/BP_LevelManager.ArrayOfPlayerProfile` _localarrayofplayerprofiles_2 (`.GameInstanceReference` (`self.GameInstanceReference`)))
              (`Widget.RemoveFromParent` (`.CreateNewProfileMenuReference` (`self.CreateNewProfileMenuReference`)))
              (`KismetSystemLibrary.CollectGarbage`))))))))

(fn `UserConstructionScript`)