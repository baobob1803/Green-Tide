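; Floating damage number actor that shows a damage value as world-space text and then removes itself.
; On BeginPlay it sizes and colors the text render component by whether the hit is critical, with criticals larger and red, then writes the integer damage.
; A timeline moves the text upward by adding a relative Z offset each update and destroys the actor when finished.
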(event `self.ReceiveBeginPlay`
  (set `self.Value` (struct :`R` 1.0 :`G` 1.0 :`B` 1.0 :`A` 1.0))
  (if (`self.DamageIsCritical`)
    (`TextRenderComponent.SetWorldSize` (`self.DamageDisplayer`) 100.0)
    (set `self.Value` (struct :`R` 1.0 :`B` 0.025124 :`A` 1.0))
    (else
      (`TextRenderComponent.SetWorldSize` (`self.DamageDisplayer`) 50.0)
      (set `self.Value` (struct :`R` 1.0 :`G` 1.0 :`B` 1.0 :`A` 1.0))))
  (`TextRenderComponent.SetTextRenderColor` (`self.DamageDisplayer`) (`KismetMathLibrary.Conv_LinearColorToColor` (`self.Value`)))
  (`TextRenderComponent.K2_SetText` (`self.DamageDisplayer`) (`KismetTextLibrary.Conv_IntToText` (`self.DamageToDisplay`) false true 0 99999))
  (bind (_direction _floatup) (`Timeline|MovingText` :!via `PlayFromStart`)
    (:`Update`
      (`SceneComponent.K2_AddRelativeLocation` (`self.DamageDisplayer`) (`KismetMathLibrary.MakeVector` 0.0 0.0 _floatup) false false))
    (:`Finished`
      (`self.K2_DestroyActor`))))

(fn `UserConstructionScript`)