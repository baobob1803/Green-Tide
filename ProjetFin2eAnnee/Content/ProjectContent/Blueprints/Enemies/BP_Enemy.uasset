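; Orc melee enemy for wave combat that attacks the player character and derives health, defense, damage and XP reward from its level and tier.
; Tick triggers cooldown-gated attacks in range, using a delayed forward sphere overlap, with a debug sphere drawn, to apply damage.
; Taking damage causes knockback via its AI controller and impulse, spawns damage text and subtracts health.
; A shared death-check macro plays the death animation before WaveManager removes the unit.
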(event Custom|AttackPlayer
  (bind _returnvalue (Transformation|GetActorTransform))
  (bind _charactermovement (Variables|Character|GetCharacterMovement))
  (bind _capsulecomponent (Variables|Collision|GetCapsuleComponent))
  (bind _maxdist (Variables|Default|GetMaxDist))
  (bind _returnvalue_2 (Math|Vector|GetForwardVector _capsulecomponent))
  (bind _returnvalue_3 (* _maxdist 1.75))
  (bind _returnvalue_4 (* _returnvalue_2 _returnvalue_3))
  (bind _returnvalue_5 (+ (.location _returnvalue) _returnvalue_4))
  ;[1 1 1] Attack
  (bind _ast_pose_orc__1__skeleton_anim_blueprint (Utilities|Casting|CastToT_Pose_ORC__1__Skeleton_AnimBlueprint (Components|SkeletalMesh|GetAnimInstance (Variables|Character|GetMesh))))
  (Variables|/Game/ProjectContent/Assets/Enemy/T_Pose_ORC__1__Skeleton_AnimBlueprint.T_Pose_ORC__1__Skeleton_AnimBlueprint_C|SetRunning _ast_pose_orc__1__skeleton_anim_blueprint false)
  (Variables|/Game/ProjectContent/Assets/Enemy/T_Pose_ORC__1__Skeleton_AnimBlueprint.T_Pose_ORC__1__Skeleton_AnimBlueprint_C|SetAttack _ast_pose_orc__1__skeleton_anim_blueprint true)
  (Variables|/Script/Engine.CharacterMovementComponent|SetMaxWalkSpeed _charactermovement 3e+02)
  (Variables|Default|SetattackCooldown (Variables|Default|GetattackTimer))
  (Utilities|DeadCheck&AnimPlay
    (:Dead
      (Default|DestroyUnite (Variables|References|GetwaveManager) self (Math|Conversions|ToFloat(Integer) (Variables|Attribute|GetxpReward)) :!label _label))
    (:NotDead
      (Utilities|FlowControl|Delay 0.8)
      (Utilities|DeadCheck&AnimPlay
        (:Dead
          (goto _label))
        (:NotDead
          (Rendering|Debug|DrawDebugSphere _returnvalue_5 5e+01 25 "(R=1.000000,G=0.000000,B=0.000000,A=1.000000)" 1.0)
          (bind (_outactors _returnvalue_6) (Collision|SphereOverlapActors _returnvalue_5 5e+01 (Utilities|Array|MakeArray "ObjectTypeQuery3") "/Game/ProjectContent/BP_Character_Master.BP_Character_Master_C"))
          (if _returnvalue_6
            (bind _asbp_character_master (Utilities|Casting|CastToBP_Character_Master (Utilities|Array|Get(acopy) _outactors)))
            (Game|Damage|ApplyDamage _asbp_character_master (Variables|Attribute|GetDamageInflicted) 0 self))
          (Variables|/Script/Engine.CharacterMovementComponent|SetMaxWalkSpeed _charactermovement 6e+02)
          (bind _ast_pose_orc__1__skeleton_anim_blueprint_2 (Utilities|Casting|CastToT_Pose_ORC__1__Skeleton_AnimBlueprint (Components|SkeletalMesh|GetAnimInstance (Variables|Character|GetMesh))))
          (Variables|/Game/ProjectContent/Assets/Enemy/T_Pose_ORC__1__Skeleton_AnimBlueprint.T_Pose_ORC__1__Skeleton_AnimBlueprint_C|SetAttack _ast_pose_orc__1__skeleton_anim_blueprint_2 false)
          (Variables|/Game/ProjectContent/Assets/Enemy/T_Pose_ORC__1__Skeleton_AnimBlueprint.T_Pose_ORC__1__Skeleton_AnimBlueprint_C|SetRunning _ast_pose_orc__1__skeleton_anim_blueprint_2 true))))))

(event Custom|Knockback
  ;[1 1 1] Knock back
  (bind _asaic_enemy (Utilities|Casting|CastToAIC_Enemy (AI|GetAIController self)))
  (Variables|/Game/ProjectContent/Enemies/AIC_Enemy.AIC_Enemy_C|SetCanMove _asaic_enemy false)
  (Physics|AddImpulse (Variables|Character|GetCharacterMovement) (* (Math|Vector|GetForwardVector (Variables|Collision|GetCapsuleComponent)) -3.5e+03) true)
  (Utilities|FlowControl|Delay 0.2)
  (Variables|/Game/ProjectContent/Enemies/AIC_Enemy.AIC_Enemy_C|SetCanMove _asaic_enemy true))

(event EventTick
  (params (DeltaSeconds :type Float%20%28single-precision%29))
  (if (not (Variables|States|GetDead))
    (if (and (<= (Math|Vector|Distance(Vector) (.location (Transformation|GetActorTransform)) (.location (Transformation|GetActorTransform (Variables|References|Getplayer)))) (* (Variables|Default|GetMaxDist) 1.75)) (<= (Variables|Default|GetattackCooldown) 0.0))
      (CallFunction|AttackPlayer)
      (else
        (Variables|Default|SetattackCooldown (- (Variables|Default|GetattackCooldown) DeltaSeconds))))))

(event Game|Damage|EventAnyDamage
  (params (Damage :type Float%20%28single-precision%29) (DamageType :type Damage%20Type%20Object%20Reference) (InstigatedBy :type Controller%20Object%20Reference) (DamageCauser :type Actor%20Object%20Reference))
  (bind _returnvalue (Math|Float|Truncate Damage))
  (bind _capsulecomponent (Variables|Collision|GetCapsuleComponent))
  ;[1 1 1] Damage
  (CallFunction|Knockback)
  (Game|SpawnActorfromClass "/Game/ProjectContent/Blueprints/Enemies/Text_Damage.Text_Damage_C" (Math|Transform|MakeTransform (+ (Transformation|GetWorldLocation (Variables|Character|GetMesh)) "0, 0,350.000000") (Transformation|GetWorldRotation (Variables|/Game/ProjectContent/BP_Character_Master.BP_Character_Master_C|GetFollowCamera (Variables|References|Getplayer))) "1,1,1") "Undefined" 0 _returnvalue (Variables|Default|GetIsBlowCritical) 0)
  (Variables|Attribute|SethealthPoint (- (Variables|Attribute|GethealthPoint) _returnvalue))
  (Variables|States|SetDead (<= (Variables|Attribute|GethealthPoint) 0))
  (Collision|SetCollisionObjectType _capsulecomponent "ECC_Destructible")
  (Physics|SetEnableGravity _capsulecomponent false)
  (Utilities|DeadCheck&AnimPlay
    (:Dead
      (Default|DestroyUnite (Variables|References|GetwaveManager) self (Math|Conversions|ToFloat(Integer) (Variables|Attribute|GetxpReward))))))

(event EventBeginPlay
  (bind _returnvalue (Actor|GetActorOfClass "/Game/ProjectContent/BP_Character_Master.BP_Character_Master_C"))
  (Variables|References|Setplayer _returnvalue)
  (CallFunction|SetEnemyCharacteristicsfromLevel))

(fn ConstructionScript)

(fn SetEnemyCharacteristicsfromLevel
  (bind _enemytier (CallFunction|GetRightEnemyTierfromLevel (Variables|Attribute|GetenemyLevel)))
  (switch string _enemytier
    (:Tier1
      (LocalVariables|SetTierMultiplier 27))
    (:Tier2
      (LocalVariables|SetTierMultiplier 60))
    (:Tier3
      (LocalVariables|SetTierMultiplier 300)))
  (CallFunction|SetAttributesfromTier (Variables|Attribute|GetenemyLevel) (LocalVariables|GetTierMultiplier)))

(fn GetRightEnemyTierfromLevel
  (params (EnemyLevel :type Integer))
  (Math|Integer|CompareInt EnemyLevel 11
    (:>
      (Math|Integer|CompareInt EnemyLevel 51 :!label _label
        (:>
          (LocalVariables|SetTierName "Tier3" :!label _label_2))
        (:==
          (goto _label_2))
        (:<
          (LocalVariables|SetTierName "Tier2"))))
    (:==
      (goto _label))
    (:<
      (LocalVariables|SetTierName "Tier1")))
  (return (LocalVariables|GetTierName)))

(fn SetAttributesfromTier
  (params (EnemyLevel :type Integer) (TierMultiplier :type Integer))
  (Variables|Attribute|SethealthPoint (* EnemyLevel TierMultiplier))
  (Variables|Attribute|SetdefenseValue (Math|Float|Round (|((Level*TierMultiplier)/1.700000) EnemyLevel TierMultiplier)))
  (Variables|Attribute|SetDamageInflicted (|((Level*5)+(Level*1.500000)) EnemyLevel))
  (Variables|Attribute|SetxpReward (|(10+Level) EnemyLevel)))