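; BP_CharacterInfo holds player character attributes and upgrades them in what appears to be a level-up step.
; UpgradePlayerStats raises six enum-keyed entries in DictOfAttributes through UpOneStats, adding each one's flat increment from DictOfAttributesScalingValue.
; It then subtracts one attribute from another, like a threshold from an accumulated total, and grows that threshold by 5 percent, so the requirement compounds with each upgrade.
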(fn `UpgradePlayerStats`
  (bind _dictofattributes (`self.DictOfAttributes`))
  (bind _dictofattributesscalingvalue (`self.DictOfAttributesScalingValue`))
  (bind _value (`BlueprintMapLibrary.Map_Find` _dictofattributes "NewEnumerator18"))
  (bind _value_2 (`BlueprintMapLibrary.Map_Find` _dictofattributes "NewEnumerator17"))
  (bind _attributevalue (`/Game/ProjectContent/Blueprints/04_PlayerLinked/BP_Attribute.AttributeValue` _value))
  (`self.UpOneStats` (`BlueprintMapLibrary.Map_Find` _dictofattributes "NewEnumerator0") (`BlueprintMapLibrary.Map_Find` _dictofattributesscalingvalue "NewEnumerator0"))
  (`self.UpOneStats` (`BlueprintMapLibrary.Map_Find` _dictofattributes "NewEnumerator1") (`BlueprintMapLibrary.Map_Find` _dictofattributesscalingvalue "NewEnumerator1"))
  (`self.UpOneStats` (`BlueprintMapLibrary.Map_Find` _dictofattributes "NewEnumerator3") (`BlueprintMapLibrary.Map_Find` _dictofattributesscalingvalue "NewEnumerator3"))
  (`self.UpOneStats` (`BlueprintMapLibrary.Map_Find` _dictofattributes "NewEnumerator4") (`BlueprintMapLibrary.Map_Find` _dictofattributesscalingvalue "NewEnumerator4"))
  (`self.UpOneStats` (`BlueprintMapLibrary.Map_Find` _dictofattributes "NewEnumerator5") (`BlueprintMapLibrary.Map_Find` _dictofattributesscalingvalue "NewEnumerator5"))
  (`self.UpOneStats` (`BlueprintMapLibrary.Map_Find` _dictofattributes "NewEnumerator2") (`BlueprintMapLibrary.Map_Find` _dictofattributesscalingvalue "NewEnumerator2"))
  (set `/Game/ProjectContent/Blueprints/04_PlayerLinked/BP_Attribute.AttributeValue` (- (`/Game/ProjectContent/Blueprints/04_PlayerLinked/BP_Attribute.AttributeValue` _value_2) _attributevalue) _value_2)
  (set `/Game/ProjectContent/Blueprints/04_PlayerLinked/BP_Attribute.AttributeValue` (* _attributevalue 1.05) _value))

(fn `UpOneStats`
  (params (ValueToScale :type "/Game/ProjectContent/Blueprints/04_PlayerLinked/BP_Attribute Object Reference") (ScallingValue :type "Float (double-precision)"))
  (set `/Game/ProjectContent/Blueprints/04_PlayerLinked/BP_Attribute.AttributeValue` (+ (`/Game/ProjectContent/Blueprints/04_PlayerLinked/BP_Attribute.AttributeValue` ValueToScale) ScallingValue) ValueToScale))