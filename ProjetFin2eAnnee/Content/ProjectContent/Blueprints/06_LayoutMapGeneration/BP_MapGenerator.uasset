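; BP_MapGenerator builds a random room layout on BeginPlay from pre-placed movable walls and Floor-tagged meshes.
; It spawns a room per floor chunk, using box traces to find walls and classify rooms.
; Walls open randomly until no room is sealed, repeating cumulatively until a graph traversal reaches 25 rooms.
; It then teleports the player into a middle room, moves the navmesh bounds and spawns wave, battle and next-room actors.
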(event `CreatingMapLayout`
  ;[1 1 1] Comment
  (`self.InitializeBaseLayoutEntities`)
  (`self.GenerateACorrectLayout`)
  (`self.DefineARandomSpawnPointForThePlayer`)
  (`self.Update Nav Mesh`))

(event `self.ReceiveBeginPlay`
  ;[1 1 1] Comment
  (`self.CreatingMapLayout`)
  (`self.InitializeDefaultSceneActors`))

(fn `CastRaysToFindWallsForEachRoom`
  (params (`Array of Rooms Ref` :type "Array of /Game/ProjectContent/Blueprints/06_LayoutMapGeneration/BP_ActorRoom Object Reference (by ref)"))
  (locals (HitElements :type "Array of HitResult Structure"))
  (for _array_element `Array of Rooms Ref`
    (`|ExecutionSequence`
      (:`then_0`
        (bind _raycastoriginmesh (`/Game/ProjectContent/Blueprints/06_LayoutMapGeneration/BP_ActorRoom.RayCastOriginMesh` _array_element))
        (bind (_returnvalue_x _returnvalue_y _returnvalue_z) (`KismetMathLibrary.BreakVector` (`SceneComponent.K2_GetComponentLocation` _raycastoriginmesh)))
        (bind _array (`|MakeArray` _array_element :!type "Actor Object Reference"))
        (bind _outhits (`KismetSystemLibrary.BoxTraceMulti` (`KismetMathLibrary.MakeVector` _returnvalue_x _returnvalue_y _returnvalue_z) (`KismetMathLibrary.MakeVector` (+ _returnvalue_x 750.0) _returnvalue_y _returnvalue_z) (0.0 0.0 0.0) (struct) "TraceTypeQuery1" false _array))
        (for _array_element_2 _outhits
          (if (`KismetMathLibrary.ClassIsChildOf` (`GameplayStatics.GetObjectClass` (`.HitActor` (`GameplayStatics.BreakHitResult` _array_element_2))) "/Game/ProjectContent/Blueprints/06_LayoutMapGeneration/BP_MovableWall.BP_MovableWall_C")
            (bind _asbp_movable_wall (cast `/Game/ProjectContent/Blueprints/06_LayoutMapGeneration/BP_MovableWall` (`.HitActor` (`GameplayStatics.BreakHitResult` _array_element_2))))
            (bind _array_of_room_walls (`/Game/ProjectContent/Blueprints/06_LayoutMapGeneration/BP_ActorRoom.Array Of Room Walls` _array_element))
            (`KismetArrayLibrary.Array_Add` _array_of_room_walls _asbp_movable_wall))))
      (:`then_1`
        (bind _outhits_2 (`KismetSystemLibrary.BoxTraceMulti` (`KismetMathLibrary.MakeVector` _returnvalue_x _returnvalue_y _returnvalue_z) (`KismetMathLibrary.MakeVector` (+ _returnvalue_x -750.0) _returnvalue_y _returnvalue_z) (0.0 0.0 0.0) (struct) "TraceTypeQuery1" false _array))
        (for _array_element_3 _outhits_2
          (if (`KismetMathLibrary.ClassIsChildOf` (`GameplayStatics.GetObjectClass` (`.HitActor` (`GameplayStatics.BreakHitResult` _array_element_3))) "/Game/ProjectContent/Blueprints/06_LayoutMapGeneration/BP_MovableWall.BP_MovableWall_C")
            (bind _asbp_movable_wall_2 (cast `/Game/ProjectContent/Blueprints/06_LayoutMapGeneration/BP_MovableWall` (`.HitActor` (`GameplayStatics.BreakHitResult` _array_element_3))))
            (`KismetArrayLibrary.Array_Add` _array_of_room_walls _asbp_movable_wall_2))))
      (:`then_2`
        (bind (_returnvalue_x_2 _returnvalue_y_2 _returnvalue_z_2) (`KismetMathLibrary.BreakVector` (`SceneComponent.K2_GetComponentLocation` _raycastoriginmesh)))
        (bind _outhits_3 (`KismetSystemLibrary.BoxTraceMulti` (`KismetMathLibrary.MakeVector` _returnvalue_x_2 _returnvalue_y_2 _returnvalue_z_2) (`KismetMathLibrary.MakeVector` _returnvalue_x_2 (+ _returnvalue_y_2 750.0) _returnvalue_z_2) (0.0 0.0 0.0) (struct) "TraceTypeQuery1" false _array))
        (for _array_element_4 _outhits_3
          (if (`KismetMathLibrary.ClassIsChildOf` (`GameplayStatics.GetObjectClass` (`.HitActor` (`GameplayStatics.BreakHitResult` _array_element_4))) "/Game/ProjectContent/Blueprints/06_LayoutMapGeneration/BP_MovableWall.BP_MovableWall_C")
            (bind _asbp_movable_wall_3 (cast `/Game/ProjectContent/Blueprints/06_LayoutMapGeneration/BP_MovableWall` (`.HitActor` (`GameplayStatics.BreakHitResult` _array_element_4))))
            (`KismetArrayLibrary.Array_Add` _array_of_room_walls _asbp_movable_wall_3))))
      (:`then_3`
        (bind _outhits_4 (`KismetSystemLibrary.BoxTraceMulti` (`KismetMathLibrary.MakeVector` _returnvalue_x_2 _returnvalue_y_2 _returnvalue_z_2) (`KismetMathLibrary.MakeVector` _returnvalue_x_2 (+ _returnvalue_y_2 -750.0) _returnvalue_z_2) (0.0 0.0 0.0) (struct) "TraceTypeQuery1" false _array))
        (for _array_element_5 _outhits_4
          (if (`KismetMathLibrary.ClassIsChildOf` (`GameplayStatics.GetObjectClass` (`.HitActor` (`GameplayStatics.BreakHitResult` _array_element_5))) "/Game/ProjectContent/Blueprints/06_LayoutMapGeneration/BP_MovableWall.BP_MovableWall_C")
            (bind _asbp_movable_wall_4 (cast `/Game/ProjectContent/Blueprints/06_LayoutMapGeneration/BP_MovableWall` (`.HitActor` (`GameplayStatics.BreakHitResult` _array_element_5))))
            (`KismetArrayLibrary.Array_Add` _array_of_room_walls _asbp_movable_wall_4))))
      (:`then_4`
        (`/Engine/EditorBlueprintResources/StandardMacros.CompareInt` (`KismetArrayLibrary.Array_Length` (`/Game/ProjectContent/Blueprints/06_LayoutMapGeneration/BP_ActorRoom.Array Of Room Walls` _array_element)) 3
          (:`>`
            (set `/Game/ProjectContent/Blueprints/06_LayoutMapGeneration/BP_ActorRoom.TypeOfRoom` "NewEnumerator2" _array_element))
          (:`==`
            (set `/Game/ProjectContent/Blueprints/06_LayoutMapGeneration/BP_ActorRoom.TypeOfRoom` "NewEnumerator1" _array_element))
          (:`<`
            (set `/Game/ProjectContent/Blueprints/06_LayoutMapGeneration/BP_ActorRoom.TypeOfRoom` "NewEnumerator0" _array_element))))))
  (for _array_element_6 `Array of Rooms Ref`
    (`SceneComponent.SetVisibility` (`/Game/ProjectContent/Blueprints/06_LayoutMapGeneration/BP_ActorRoom.RayCastOriginMesh` _array_element_6) false true)))

(fn `DefineARandomSpawnPointForThePlayer`
  (locals (`Random Room` :type "/Game/ProjectContent/Blueprints/06_LayoutMapGeneration/BP_ActorRoom Object Reference"))
  ;[1 1 1] Getting a random room and saving it in a local variable
  (bind _output_get (set `local.Random Room` (`KismetArrayLibrary.Array_Random` (`self.Array Of Instanciated Rooms`)) :!label _label))
  ;[1 1 1] Anti Edge-Spawn
  (if (`|EnumEquality` (`/Game/ProjectContent/Blueprints/06_LayoutMapGeneration/BP_ActorRoom.TypeOfRoom` _output_get) "NewEnumerator2")
    ;[1 1 1] Teleport Character to Defined Spawn
    (bind _returnvalue (`GameplayStatics.GetActorOfClass` "/Game/ProjectContent/BP_Character_Master.BP_Character_Master_C"))
    (`self.K2_SetActorTransform` _returnvalue (`self.GetTransform` (`local.Random Room`)) false false)
    (else
      (goto _label))))

(fn `GenerateACorrectLayout`
  (`self.WallRandomization` :!label _label)
  (`self.GetAccessibleRoomForEachRoom`)
  (bind _layout_is_correct (`self.Verify Layout`))
  (if (not _layout_is_correct)
    (`self.ResetLayout`)
    (goto _label)))

(fn `Get Neighboor Rooms for Each Room`
  (for (_array_element _array_index) (`self.Array Of Instanciated Rooms`)
    (for _array_element_2 (`/Game/ProjectContent/Blueprints/06_LayoutMapGeneration/BP_ActorRoom.Array Of Room Walls` _array_element)
      (for (_array_element_3 _array_index_2) (`self.Array Of Instanciated Rooms`)
        (if (`KismetArrayLibrary.Array_Contains` (`/Game/ProjectContent/Blueprints/06_LayoutMapGeneration/BP_ActorRoom.Array Of Room Walls` _array_element_3) _array_element_2)
          (if (not (== _array_index_2 _array_index))
            (`KismetArrayLibrary.Array_Add` (`/Game/ProjectContent/Blueprints/06_LayoutMapGeneration/BP_ActorRoom.ListOfOpenedAdjacentRooms` _array_element) _array_element_3)))))))

(fn `GetAccessibleRoomForEachRoom`
  (for (_array_element _array_index) (`self.Array Of Instanciated Rooms`)
    (for _array_element_2 (`/Game/ProjectContent/Blueprints/06_LayoutMapGeneration/BP_ActorRoom.Array Of Room Walls` _array_element)
      (if (not (`SceneComponent.IsVisible` (`/Game/ProjectContent/Blueprints/06_LayoutMapGeneration/BP_MovableWall.WallMesh` _array_element_2)))
        (for (_array_element_3 _array_index_2) (`self.Array Of Instanciated Rooms`)
          (if (`KismetArrayLibrary.Array_Contains` (`/Game/ProjectContent/Blueprints/06_LayoutMapGeneration/BP_ActorRoom.Array Of Room Walls` _array_element_3) _array_element_2)
            (if (not (== _array_index_2 _array_index))
              (`KismetArrayLibrary.Array_Add` (`/Game/ProjectContent/Blueprints/06_LayoutMapGeneration/BP_ActorRoom.ListOfOpenedAdjacentRooms` _array_element) _array_element_3))))))))

(fn `GetAllFloorChunksPositions`
  (returns (`Array Of Floor Chunks Transform` :type "Array of Transform Structure"))
  (locals (FoundTransformArray :type "Array of Transform Structure"))
  (bind _outactors (`GameplayStatics.GetAllActorsOfClassWithTag` "/Script/Engine.StaticMeshActor" "Floor"))
  (for _array_element _outactors
    (`KismetArrayLibrary.Array_Add` (`local.FoundTransformArray`) (`self.GetTransform` _array_element)))
  (return (`local.FoundTransformArray`)))

(fn `InitializeBaseLayoutEntities`
  (locals (NewLocalVar_1 :type "Array of /Game/ProjectContent/Blueprints/06_LayoutMapGeneration/BP_ActorRoom Object Reference"))
  ;[1 1 1] Finding All Movable Walls pre-placed in the Scene
  (bind _outactors (`GameplayStatics.GetAllActorsOfClass` "/Game/ProjectContent/Blueprints/06_LayoutMapGeneration/BP_MovableWall.BP_MovableWall_C"))
  (set `self.List Of Movable Walls` _outactors)
  ;[1 1 1] Getting all floor chunk positions and saving them.
  (bind _array_of_floor_chunks_transform (`self.GetAllFloorChunksPositions`))
  (bind _output_get (set `self.Array Of Floor Chunks Transform` _array_of_floor_chunks_transform))
  ;[1 1 1] Spawn Abstract Room Entities using the position of each floor chunk.
  (bind _arrayofinstanciatedroomactors (`self.SpawnRoomActor` _output_get))
  (bind _output_get_2 (set `self.Array Of Instanciated Rooms` _arrayofinstanciatedroomactors))
  (`self.CastRaysToFindWallsForEachRoom` _output_get_2))

(fn `InitializeDefaultSceneActors`
  (bind _spawn_transform (`self.Spawn Transform`))
  (`|SpawnActorFromClass` "/Game/ProjectContent/Enemies/BP_RealWaveManager.BP_RealWaveManager_C" _spawn_transform "AdjustIfPossibleButAlwaysSpawn" "OverrideRootScale" null null)
  (`|SpawnActorFromClass` "/Game/ProjectContent/Blueprints/BP_BattleManager.BP_BattleManager_C" _spawn_transform "AdjustIfPossibleButAlwaysSpawn" "OverrideRootScale" null null)
  (`|SpawnActorFromClass` "/Game/ProjectContent/Blueprints/BP_NextRoom.BP_NextRoom_C" (`KismetArrayLibrary.Array_Random` (`self.Array Of Floor Chunks Transform`)) "AdjustIfPossibleButAlwaysSpawn" "OverrideRootScale" null null))

(fn `IsRoomHermetic`
  (params (ArrayOfWallsToCheck :type "Array of /Game/ProjectContent/Blueprints/06_LayoutMapGeneration/BP_MovableWall Object Reference"))
  (returns (IsRoomHermetic :type Boolean))
  (locals (AtLeastOneWallIsOpened :type Boolean))
  (for _array_element ArrayOfWallsToCheck
    (if (not (`PrimitiveComponent.K2_IsCollisionEnabled` (`/Game/ProjectContent/Blueprints/06_LayoutMapGeneration/BP_MovableWall.WallMesh` _array_element)))
      (set `local.AtLeastOneWallIsOpened` true)))
  (if (`local.AtLeastOneWallIsOpened`)
    (return false)
    (else
      (for _array_element_2 ArrayOfWallsToCheck
        (set `/Game/ProjectContent/Blueprints/06_LayoutMapGeneration/BP_MovableWall.HasBeenProcessed` false _array_element_2))
      (return true))))

(fn `ResetLayout`
  ;[1 1 1] Resetting Useful Variables
  (for _array_element (`self.List Of Movable Walls`)
    (set `/Game/ProjectContent/Blueprints/06_LayoutMapGeneration/BP_MovableWall.HasBeenProcessed` false _array_element))
  (for _array_element_2 (`self.Array Of Instanciated Rooms`)
    (set `/Game/ProjectContent/Blueprints/06_LayoutMapGeneration/BP_ActorRoom.RoomWasAccessed` false _array_element_2)))

(fn `SpawnRoomActor`
  (params (Array :type "Array of Transform Structure"))
  (returns (ArrayOfInstanciatedRoomActors :type "Array of /Game/ProjectContent/Blueprints/06_LayoutMapGeneration/BP_ActorRoom Object Reference"))
  (locals (LocalArrayOfRoomActor :type "Array of /Game/ProjectContent/Blueprints/06_LayoutMapGeneration/BP_ActorRoom Object Reference"))
  (bind _localarrayofroomactor (`local.LocalArrayOfRoomActor`))
  (for _array_element Array
    (bind _returnvalue (`|SpawnActorFromClass` "/Game/ProjectContent/Blueprints/06_LayoutMapGeneration/BP_ActorRoom.BP_ActorRoom_C" (`KismetMathLibrary.MakeTransform` (`KismetMathLibrary.MakeVector` (.x (.location _array_element)) (.y (.location _array_element)) (+ (.z (.location _array_element)) 50.0)) (.rotation _array_element) (.scale _array_element)) "AlwaysSpawn" "OverrideRootScale" null null))
    (`KismetArrayLibrary.Array_Add` _localarrayofroomactor _returnvalue))
  (return _localarrayofroomactor))

(fn `Update Nav Mesh`
  (locals (`Nav Mesh bounds Class ref` :type "NavMeshBoundsVolume Class Reference"))
  (bind _returnvalue (`GameplayStatics.GetActorOfClass` "/Script/NavigationSystem.NavMeshBoundsVolume"))
  (set `local.Nav Mesh bounds Class ref` (`GameplayStatics.GetObjectClass` _returnvalue))
  (`self.K2_SetActorLocation` _returnvalue (0.0 2100.0 6.0) false false))

(fn `UserConstructionScript`)

(fn `Verify Layout`
  (returns (`Layout Is Correct` :type Boolean))
  (locals (RoomToExplore :type "Array of /Game/ProjectContent/Blueprints/06_LayoutMapGeneration/BP_ActorRoom Object Reference") (NumberOfExploredRoom :type Integer :default 0) (NewLocalVar_0 :type "/Game/ProjectContent/Blueprints/06_LayoutMapGeneration/BP_ActorRoom Object Reference") (LocalArrayOfRooms :type "Array of /Game/ProjectContent/Blueprints/06_LayoutMapGeneration/BP_ActorRoom Object Reference"))
  (bind _localarrayofrooms (`local.LocalArrayOfRooms`))
  (bind _localarrayofrooms_2 (`local.LocalArrayOfRooms`))
  (bind _output (`|GetArrayItem` (`local.LocalArrayOfRooms`)))
  ;[1 1 1] Alogithme de passage en profondeur
  ;;[1 1 1] Initialisation de l'algorithme
  (bind _returnvalue (`KismetArrayLibrary.Array_Add` _localarrayofrooms (`|GetArrayItem` (`self.Array Of Instanciated Rooms`))))
  (bind _output_2 (`|GetArrayItem` _localarrayofrooms _returnvalue))
  (set `/Game/ProjectContent/Blueprints/06_LayoutMapGeneration/BP_ActorRoom.RoomWasAccessed` true _output_2)
  (`/Engine/EditorBlueprintResources/StandardMacros.IncrementInt` (`local.NumberOfExploredRoom`)
    (:`  `
      (for _array_element (`/Game/ProjectContent/Blueprints/06_LayoutMapGeneration/BP_ActorRoom.ListOfOpenedAdjacentRooms` _output_2)
        (if (not (`/Game/ProjectContent/Blueprints/06_LayoutMapGeneration/BP_ActorRoom.RoomWasAccessed` _array_element))
          (`KismetArrayLibrary.Array_Add` (`local.LocalArrayOfRooms`) _array_element)))
      (`KismetArrayLibrary.Array_RemoveItem` (`local.LocalArrayOfRooms`) _output_2)
      ;;[0 1 0.6755] Boucle de l'algorithme
      (set `/Game/ProjectContent/Blueprints/06_LayoutMapGeneration/BP_ActorRoom.RoomWasAccessed` true _output :!label _label)
      (`/Engine/EditorBlueprintResources/StandardMacros.IncrementInt` (`local.NumberOfExploredRoom`)
        (:`  `
          (for _array_element_2 (`/Game/ProjectContent/Blueprints/06_LayoutMapGeneration/BP_ActorRoom.ListOfOpenedAdjacentRooms` _output)
            (if (`KismetArrayLibrary.Array_Contains` _localarrayofrooms_2 _array_element_2)
              _
              (elif (not (`/Game/ProjectContent/Blueprints/06_LayoutMapGeneration/BP_ActorRoom.RoomWasAccessed` _array_element_2))
                (`KismetArrayLibrary.Array_Add` _localarrayofrooms_2 _array_element_2))))
          (`KismetArrayLibrary.Array_RemoveItem` _localarrayofrooms_2 _output)
          ;;[1 0.3167 0.09549] Condition d'arrêt
          (if (== (`KismetArrayLibrary.Array_Length` _localarrayofrooms_2) 0)
            ;;[0.5849 1 0] Condition De validité
            (if (>= (`local.NumberOfExploredRoom`) 25)
              (return true)
              (else
                (return false)))
            (else
              (goto _label))))))))

(fn `WallRandomization`
  (for _array_element (`self.Array Of Instanciated Rooms`)
    (switch `/Game/ProjectContent/Blueprints/06_LayoutMapGeneration/TypeOfRoomsEnums` (`/Game/ProjectContent/Blueprints/06_LayoutMapGeneration/BP_ActorRoom.TypeOfRoom` _array_element)
      (:`NewEnumerator0`
        _)
      (:`NewEnumerator1`
        _)
      (:`NewEnumerator2`
        _))
    (bind _array_of_room_walls (`/Game/ProjectContent/Blueprints/06_LayoutMapGeneration/BP_ActorRoom.Array Of Room Walls` _array_element))
    (for _array_element_2 _array_of_room_walls :!label _label
      (if (< (`KismetMathLibrary.RandomFloat`) 0.05)
        (bind _wallmesh (`/Game/ProjectContent/Blueprints/06_LayoutMapGeneration/BP_MovableWall.WallMesh` _array_element_2))
        (`PrimitiveComponent.SetCollisionEnabled` _wallmesh "NoCollision")
        (`SceneComponent.SetVisibility` _wallmesh false true))
      (set `/Game/ProjectContent/Blueprints/06_LayoutMapGeneration/BP_MovableWall.HasBeenProcessed` true _array_element_2))
    (bind _isroomhermetic (`self.IsRoomHermetic` _array_of_room_walls))
    (if _isroomhermetic
      (goto _label))))