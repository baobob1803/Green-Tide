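; BP_MovableWall is a wall actor with two point lights that flicker like fire; the graph contains no movement logic.
; A timeline drives both lights' color and intensity, scaled by a multiplier, and replays after a short delay each time it finishes.
; A random time chosen at BeginPlay is meant to offset the timeline's start, then is zeroed once for later loops.
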(event `self.ReceiveBeginPlay`
  (bind _pointlight (`self.PointLight`))
  (bind _pointlight1 (`self.PointLight1`))
  (set `self.NewTime` (`KismetMathLibrary.RandomFloatInRange` 0.0 4.0))
  (if (`self.hasBegun`) :!label _label
    (`|ExecutionSequence`
      (:`then_0`
        ;[1 1 1] Update Timeline
        (bind (_direction _intensity _fire_color) (`Timeline|Timeline_0` :`NewTime` (`self.NewTime`) :!via `SetNewTime` :!label _label_2)
          (:`Update`
            (bind _returnvalue (* _intensity (`self.IntensityMultiplier`)))
            (`LightComponent.SetIntensity` _pointlight _returnvalue)
            (`LightComponent.SetLightColor` _pointlight _fire_color true)
            (`LightComponent.SetIntensity` _pointlight1 _returnvalue)
            (`LightComponent.SetLightColor` _pointlight1 _fire_color true)
            ;[1 1 1] First Color and intensity Update reset start time of the timeline
            (`/Engine/EditorBlueprintResources/StandardMacros.DoOnce` false
              (:`Completed`
                (set `self.NewTime` 0.0))))
          (:`Finished`
            (`KismetSystemLibrary.Delay` 0.2)
            (goto _label))))
      (:`then_1`
        (goto _label_2 :!via `PlayFromStart`)))
    (else
      (set `self.hasBegun` true)
      (`|ExecutionSequence`
        (:`then_0`
          (goto _label_2 :!via `SetNewTime`))
        (:`then_1`
          (goto _label_2))))))

(fn `UserConstructionScript`)