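; BP_ItemGenerator builds a randomized loot item, with its level based on a dead enemy's level.
; GenerateItem constructs a random item class with a clamped level offset and a rarity from cascading rolls, which can fail to match.
; Weapon and clothing branches use class checks and casts to roll level-based stats.
; Trait selection by type and rarity is disconnected, two-handed and misc handling are unfinished, and one-handed damage divides by zero.
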(event `self.ReceiveBeginPlay`)

(fn `ConstructItem`
  (params (`Item Class Reference` :type "/Game/ProjectContent/Blueprints/ItemGenerator/ItemHierarchy/BP_Item Class Reference") (Level :type Integer) (Rarity :type "/Game/ProjectContent/Blueprints/ItemGenerator/ItemHierarchy/RarityEnum Enum" :default "NewEnumerator0"))
  (`|GenericCreateObject` `Item Class Reference` self Level Rarity))

(fn `DefineItemLevel`
  (params (A :type Integer))
  (returns (`Item Actual Level` :type Integer))
  (locals (FoundItemLevel :type Integer :default 0))
  (bind _output_get (set `local.FoundItemLevel` (+ A (`KismetMathLibrary.RandomIntegerInRange` -2 2))))
  (return (`KismetMathLibrary.Clamp` _output_get 1 100)))

(fn `DefineItemRarity`
  (returns (NewParam :type "/Game/ProjectContent/Blueprints/ItemGenerator/ItemHierarchy/RarityEnum Enum"))
  (locals (FoundRarity :type "/Game/ProjectContent/Blueprints/ItemGenerator/ItemHierarchy/RarityEnum Enum"))
  (bind _returnvalue (`KismetMathLibrary.RandomIntegerInRange` 1 100))
  (if (< _returnvalue 5)
    (set `local.FoundRarity` "NewEnumerator3")
    (return (`local.FoundRarity`))
    (elif (< _returnvalue 15)
      (set `local.FoundRarity` "NewEnumerator2")
      (return (`local.FoundRarity`))
      (elif (< _returnvalue 35)
        (set `local.FoundRarity` "NewEnumerator1")
        (return (`local.FoundRarity`))
        (elif (< _returnvalue 60)
          (set `local.FoundRarity` "NewEnumerator0")
          (return (`local.FoundRarity`))
          (else
            (`KismetSystemLibrary.PrintString` "Bah dégage alors")))))))

(fn `Generate Item`
  (params (DeadEnemyLevel :type Integer))
  (bind _found_class (`self.GetRandomItemClassToSpawn`))
  (bind _item_actual_level (`self.DefineItemLevel` DeadEnemyLevel))
  (bind _newparam (`self.DefineItemRarity`))
  (bind _returnvalue (`|GenericCreateObject` _found_class self _item_actual_level _newparam))
  (set `self.CurrentItem` _returnvalue)
  (bind (_asbp_weapon _isitemweapon) (`self.Get Item As Weapon` (`self.CurrentItem`)))
  (if _isitemweapon
    (`self.HandleWeapon`)
    (`self.Get Random Traits`)
    (else
      (bind (_asbp_clothe _isitemclothe) (`self.Get Item As Clothe` (`self.CurrentItem`)))
      (if _isitemclothe
        (`self.HandleClothe` null)
        (`self.Get Random Traits`)))))

(fn `Get Item As Clothe`
  (params (CurrentEquipement :type "/Game/ProjectContent/Blueprints/ItemGenerator/ItemHierarchy/BP_Item Object Reference (by ref)"))
  (returns (`AsBP Clothe` :type "/Game/ProjectContent/Blueprints/ItemGenerator/ItemHierarchy/BP_Clothe Object Reference") (IsItemClothe :type Boolean))
  (locals (ItemIsClothe :type Boolean))
  (if (`KismetMathLibrary.ClassIsChildOf` (`GameplayStatics.GetObjectClass` CurrentEquipement) "/Game/ProjectContent/Blueprints/ItemGenerator/ItemHierarchy/BP_Clothe.BP_Clothe_C")
    (bind _asbp_clothe (cast `/Game/ProjectContent/Blueprints/ItemGenerator/ItemHierarchy/BP_Clothe` CurrentEquipement))
    (set `local.ItemIsClothe` true)
    (else
      (set `local.ItemIsClothe` false)))
  (return _asbp_clothe (`local.ItemIsClothe`)))

(fn `Get Item As Misc`
  (params (CurrentEquipement :type "/Game/ProjectContent/Blueprints/ItemGenerator/ItemHierarchy/BP_Item Object Reference (by ref)"))
  (returns (`AsBP Weapon` :type "/Game/ProjectContent/Blueprints/ItemGenerator/ItemHierarchy/BP_Weapon Object Reference") (`Item Is Not a Weapon` :type Boolean))
  (locals (ItemIsOfWeapon :type Boolean))
  (if (`KismetMathLibrary.ClassIsChildOf` (`GameplayStatics.GetObjectClass` CurrentEquipement) "/Game/ProjectContent/Blueprints/ItemGenerator/ItemHierarchy/BP_Weapon.BP_Weapon_C")
    (bind _asbp_weapon (cast `/Game/ProjectContent/Blueprints/ItemGenerator/ItemHierarchy/BP_Weapon` CurrentEquipement))
    (set `local.ItemIsOfWeapon` true)
    (else
      (set `local.ItemIsOfWeapon` false)))
  (return _asbp_weapon (`local.ItemIsOfWeapon`)))

(fn `Get Item As Weapon`
  (params (CurrentEquipement :type "/Game/ProjectContent/Blueprints/ItemGenerator/ItemHierarchy/BP_Item Object Reference (by ref)"))
  (returns (`AsBP Weapon` :type "/Game/ProjectContent/Blueprints/ItemGenerator/ItemHierarchy/BP_Weapon Object Reference") (IsItemWeapon :type Boolean))
  (locals (ItemIsOfWeapon :type Boolean))
  (if (`KismetMathLibrary.ClassIsChildOf` (`GameplayStatics.GetObjectClass` CurrentEquipement) "/Game/ProjectContent/Blueprints/ItemGenerator/ItemHierarchy/BP_Weapon.BP_Weapon_C")
    (bind _asbp_weapon (cast `/Game/ProjectContent/Blueprints/ItemGenerator/ItemHierarchy/BP_Weapon` CurrentEquipement))
    (set `local.ItemIsOfWeapon` true)
    (else
      (set `local.ItemIsOfWeapon` false)))
  (return _asbp_weapon (`local.ItemIsOfWeapon`)))

(fn `Get Random Traits`
  (locals (InitializedItem :type "/Game/ProjectContent/Blueprints/ItemGenerator/ItemHierarchy/BP_Item_Abstract Object Reference") (ArrayOfEquipementTraits :type "Array of /Game/ProjectContent/Blueprints/ItemGenerator/ItemTraitsHierarchy/BP_EquipementTrait_Abstract Class Reference"))
  (if (`KismetMathLibrary.ClassIsChildOf` (`GameplayStatics.GetObjectClass` (`self.CurrentItem`)) "/Game/ProjectContent/Blueprints/ItemGenerator/ItemHierarchy/BP_Weapon.BP_Weapon_C")
    _))

(fn `GetRandomItemClassToSpawn`
  (returns (`Found Class` :type "/Game/ProjectContent/Blueprints/ItemGenerator/ItemHierarchy/BP_Item Class Reference"))
  (bind _output_get (set `self.GeneratedItemClass` (`KismetArrayLibrary.Array_Random` (`self.ArrayOfAllItemClasses`))))
  (return _output_get))

(fn `HandleArmoredClothe`
  (params (CurrentClothe :type "/Game/ProjectContent/Blueprints/ItemGenerator/ItemHierarchy/Clothes/BP_Clothe_Abstract Object Reference"))
  (returns (NewParam :type "/Game/ProjectContent/Blueprints/ItemGenerator/ItemHierarchy/Clothes/ArmoredClothe/BP_ArmoredClothe_Abstract Object Reference"))
  (locals (CurrentArmoredClothe :type "/Game/ProjectContent/Blueprints/ItemGenerator/ItemHierarchy/Clothes/ArmoredClothe/BP_ArmoredClothe_Abstract Object Reference"))
  (bind _asbp_armored_clothe_abstract (cast `/Game/ProjectContent/Blueprints/ItemGenerator/ItemHierarchy/Clothes/ArmoredClothe/BP_ArmoredClothe_Abstract` CurrentClothe))
  (bind _output_get (set `local.CurrentArmoredClothe` _asbp_armored_clothe_abstract))
  (return _output_get))

(fn `HandleClothe`
  (params (CurrentObject :type "/Game/ProjectContent/Blueprints/ItemGenerator/ItemHierarchy/BP_Item_Abstract Object Reference"))
  (returns (NewParam :type "/Game/ProjectContent/Blueprints/ItemGenerator/ItemHierarchy/BP_Item_Abstract Object Reference"))
  (locals (RarityMultiplier :type "Float (double-precision)"))
  (bind _currentclothe (`self.CurrentClothe`))
  (bind _asbp_clothe_abstract (cast `/Game/ProjectContent/Blueprints/ItemGenerator/ItemHierarchy/Clothes/BP_Clothe_Abstract` CurrentObject))
  (bind _output_get (set `self.CurrentClothe` _asbp_clothe_abstract))
  (bind _returnvalue (`KismetMathLibrary.FTrunc` (* (* (`/Game/ProjectContent/Blueprints/ItemGenerator/ItemHierarchy/BP_Item_Abstract.ItemLevel` _output_get) (`KismetMathLibrary.RandomFloatInRange` 2.0 4.0)) 1.0)))
  (set `/Game/ProjectContent/Blueprints/ItemGenerator/ItemHierarchy/Clothes/BP_Clothe_Abstract.DefenseValue` _returnvalue _currentclothe)
  (set `/Game/ProjectContent/Blueprints/ItemGenerator/ItemHierarchy/Clothes/BP_Clothe_Abstract.HealthValue` _returnvalue _currentclothe)
  (bind _item (`self.IsClotheArmored` (`self.CurrentClothe`)))
  (return _item))

(fn `HandleNonArmoredClothe`
  (params (CurrentClothe :type "/Game/ProjectContent/Blueprints/ItemGenerator/ItemHierarchy/Clothes/BP_Clothe_Abstract Object Reference"))
  (returns (NewParam :type "/Game/ProjectContent/Blueprints/ItemGenerator/ItemHierarchy/Clothes/UnarmoredClothes/BP_UnarmoredClothe_Abstract Object Reference"))
  (locals (CurrentUnarmoredClothe :type "/Game/ProjectContent/Blueprints/ItemGenerator/ItemHierarchy/Clothes/UnarmoredClothes/BP_UnarmoredClothe_Abstract Object Reference"))
  (bind _asbp_unarmored_clothe_abstract (cast `/Game/ProjectContent/Blueprints/ItemGenerator/ItemHierarchy/Clothes/UnarmoredClothes/BP_UnarmoredClothe_Abstract` CurrentClothe))
  (set `local.CurrentUnarmoredClothe` _asbp_unarmored_clothe_abstract)
  (return (`local.CurrentUnarmoredClothe`)))

(fn `HandleOneHandedWeapon`
  (params (CurrentWeapon :type "/Game/ProjectContent/Blueprints/ItemGenerator/ItemHierarchy/BP_Weapon Object Reference (by ref)"))
  (locals (NewLocalVar_0 :type "Array of String") (CurrentOneHandedWeapon :type "/Game/ProjectContent/Blueprints/ItemGenerator/ItemHierarchy/Weapons/BP_OneHandedWeapon Object Reference"))
  (bind _asbp_one_handed_weapon (cast `/Game/ProjectContent/Blueprints/ItemGenerator/ItemHierarchy/Weapons/BP_OneHandedWeapon` CurrentWeapon))
  (bind _output_get (set `local.CurrentOneHandedWeapon` _asbp_one_handed_weapon))
  (set `/Game/ProjectContent/Blueprints/ItemGenerator/ItemHierarchy/BP_Weapon.LowerDamageValue` (/ (`/Game/ProjectContent/Blueprints/ItemGenerator/ItemHierarchy/BP_Weapon.LowerDamageValue` _output_get) 0) _output_get)
  (set `/Game/ProjectContent/Blueprints/ItemGenerator/ItemHierarchy/BP_Weapon.HigherDamageValue` (/ (`/Game/ProjectContent/Blueprints/ItemGenerator/ItemHierarchy/BP_Weapon.HigherDamageValue` _output_get) 1) _output_get))

(fn `HandleTwoHandedWeapon`
  (params (CurrentWeapon :type "/Game/ProjectContent/Blueprints/ItemGenerator/ItemHierarchy/BP_Weapon Object Reference (by ref)"))
  (returns (NewParam :type "/Game/ProjectContent/Blueprints/ItemGenerator/ItemHierarchy/Weapons/TwoHandedWeapons/BP_TwoHandedWeapons_Abstract Object Reference"))
  (locals (currentTwoHandedWeapon :type "/Game/ProjectContent/Blueprints/ItemGenerator/ItemHierarchy/Weapons/TwoHandedWeapons/BP_TwoHandedWeapons_Abstract Object Reference"))
  (set `local.currentTwoHandedWeapon` null)
  (return (`local.currentTwoHandedWeapon`)))

(fn `HandleWeapon`
  (locals (RarityMultiplier :type "Float (double-precision)" :default 0.0) (NewLocalVar_0 :type "/Game/ProjectContent/Blueprints/ItemGenerator/ItemHierarchy/RarityEnum Enum") (NewLocalVar_1 :type "/Game/ProjectContent/Blueprints/ItemGenerator/ItemHierarchy/BP_Weapon Object Reference") (SuperTemporaryWeapon :type "/Game/ProjectContent/Blueprints/ItemGenerator/ItemHierarchy/BP_Weapon Object Reference"))
  (bind _asbp_weapon (cast `/Game/ProjectContent/Blueprints/ItemGenerator/ItemHierarchy/BP_Weapon` (`self.CurrentItem`)))
  (set `/Game/ProjectContent/Blueprints/ItemGenerator/ItemHierarchy/BP_Weapon.PowerValue` (`KismetMathLibrary.FTrunc` (* (* (`/Game/ProjectContent/Blueprints/ItemGenerator/ItemHierarchy/BP_Item.ItemLevel` _asbp_weapon) (`KismetMathLibrary.RandomFloatInRange` 2.0 4.0)) 1.0)) _asbp_weapon)
  (bind _itemlevel (`/Game/ProjectContent/Blueprints/ItemGenerator/ItemHierarchy/BP_Item.ItemLevel` _asbp_weapon))
  (set `/Game/ProjectContent/Blueprints/ItemGenerator/ItemHierarchy/BP_Weapon.LowerDamageValue` (+ (`KismetMathLibrary.RandomIntegerInRange` 5 15) _itemlevel) _asbp_weapon)
  (set `/Game/ProjectContent/Blueprints/ItemGenerator/ItemHierarchy/BP_Weapon.HigherDamageValue` (+ _itemlevel (`KismetMathLibrary.RandomIntegerInRange` 16 30)) _asbp_weapon)
  (`self.IsWeaponOneHanded` _asbp_weapon))

(fn `IsClotheArmored`
  (params (CurrentClothe :type "/Game/ProjectContent/Blueprints/ItemGenerator/ItemHierarchy/Clothes/BP_Clothe_Abstract Object Reference"))
  (returns (Item :type "/Game/ProjectContent/Blueprints/ItemGenerator/ItemHierarchy/BP_Item_Abstract Object Reference"))
  (locals (`Recasted Item` :type "/Game/ProjectContent/Blueprints/ItemGenerator/ItemHierarchy/BP_Item_Abstract Object Reference"))
  (if (`KismetMathLibrary.ClassIsChildOf` (`GameplayStatics.GetObjectClass` CurrentClothe) "/Game/ProjectContent/Blueprints/ItemGenerator/ItemHierarchy/Clothes/ArmoredClothe/BP_ArmoredClothe_Abstract.BP_ArmoredClothe_Abstract_C")
    (set `/Game/ProjectContent/Blueprints/ItemGenerator/ItemHierarchy/BP_Item_Abstract.ItemIsArmoredCloth` true CurrentClothe)
    (bind _newparam (`self.HandleArmoredClothe` CurrentClothe))
    (bind _asbp_item_abstract (cast `/Game/ProjectContent/Blueprints/ItemGenerator/ItemHierarchy/BP_Item_Abstract` _newparam))
    (bind _output_get (set `local.Recasted Item` _asbp_item_abstract))
    (return _output_get)
    (else
      (set `/Game/ProjectContent/Blueprints/ItemGenerator/ItemHierarchy/BP_Item_Abstract.ItemIsArmoredCloth` false CurrentClothe)
      (bind _newparam_2 (`self.HandleNonArmoredClothe` CurrentClothe))
      (bind _asbp_item_abstract_2 (cast `/Game/ProjectContent/Blueprints/ItemGenerator/ItemHierarchy/BP_Item_Abstract` _newparam_2))
      (bind _output_get_2 (set `local.Recasted Item` _asbp_item_abstract_2))
      (return _output_get_2))))

(fn `IsWeaponOneHanded`
  (params (CurrentWeapon :type "/Game/ProjectContent/Blueprints/ItemGenerator/ItemHierarchy/BP_Weapon Object Reference (by ref)"))
  (locals (`Recasted Item` :type "/Game/ProjectContent/Blueprints/ItemGenerator/ItemHierarchy/BP_Item_Abstract Object Reference"))
  (if (`KismetMathLibrary.ClassIsChildOf` (`GameplayStatics.GetObjectClass` CurrentWeapon) "/Game/ProjectContent/Blueprints/ItemGenerator/ItemHierarchy/Weapons/BP_OneHandedWeapon.BP_OneHandedWeapon_C")
    (`self.HandleOneHandedWeapon` CurrentWeapon)
    (else
      (`self.HandleTwoHandedWeapon` CurrentWeapon))))

(fn `UserConstructionScript`)