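; BP_NextRoom is a portal actor that advances the player to the next room once the current one is completed.
; On BeginPlay it caches the wave manager and battle manager found in the level and deactivates its portal effect.
; When its static mesh is overlapped and the wave manager reports RoomCompleted, it deactivates the effect, waits briefly, then calls OnNextRoom on the battle manager.
; The overlapping actor is not filtered.
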(event `self.ReceiveBeginPlay`
  (bind _returnvalue (`GameplayStatics.GetActorOfClass` "/Game/ProjectContent/Enemies/BP_RealWaveManager.BP_RealWaveManager_C"))
  (set `self.waveManager` _returnvalue)
  (bind _returnvalue_2 (`GameplayStatics.GetActorOfClass` "/Game/ProjectContent/Blueprints/BP_BattleManager.BP_BattleManager_C"))
  (set `self.battleManager` _returnvalue_2)
  (`ActorComponent.Deactivate` (`self.PortalEffect`)))

(event `self.StaticMesh.OnComponentBeginOverlap`
  (params (OverlappedComponent :type "PrimitiveComponent Object Reference") (OtherActor :type "Actor Object Reference") (OtherComp :type "PrimitiveComponent Object Reference") (OtherBodyIndex :type Integer) (bFromSweep :type Boolean) (SweepResult :type "HitResult Structure (by ref)"))
  (if (`/Game/ProjectContent/Enemies/BP_RealWaveManager.roomCompleted` (`self.waveManager`))
    (`ActorComponent.Deactivate` (`self.PortalEffect`))
    (`KismetSystemLibrary.Delay` 0.5)
    (`/Game/ProjectContent/Blueprints/BP_BattleManager.OnNextRoom` (`self.battleManager`))))

(fn `UserConstructionScript`)