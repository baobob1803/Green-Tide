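; Manager for the village hub that runs its HUD, building screens and music.
; On BeginPlay it shows the cursor, creates the main HUD, spawns BP_ItemGenerator to fill a random-sized marketplace stock from a selected-character attribute, and starts music if enabled.
; Open/close events manage Basement (with stats, inventory, chest), Forge, Marketplace and Battlefield widgets, storing references and mostly open flags.
; Helper functions read the selected character, attributes and room level from BP_GameInstance.
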(event `PlayMusic`
  (bind _audio (`self.Audio`))
  (if (`/Game/ProjectContent/Blueprints/00_Manager/BP_GameInstance.MusicIsActive` (`self.GameInstanceRef`))
    (`AudioComponent.SetSound` _audio "/Game/ProjectContent/Assets/SoundDesign/Soundtrack/Into_the_Fog_-_2.Into_the_Fog_-_2")
    (`AudioComponent.FadeIn` (`self.Audio`) 2.0 0.07 10.0 "Linear")
    (else
      (`AudioComponent.SetSound` _audio null))))

(event `FadeOutMusic`
  (if (`/Game/ProjectContent/Blueprints/00_Manager/BP_GameInstance.MusicIsActive` (`self.GameInstanceRef`))
    (`AudioComponent.FadeOut` (`self.Audio`) 1.8 0.0 "Linear")))

(event `self.ReceiveBeginPlay`
  ;[1 1 1] Creat & reference main village HUD
  (set `PlayerController.bShowMouseCursor` true (`GameplayStatics.GetPlayerController` 0))
  (bind _returnvalue (`|CreateWidget` "/Game/ProjectContent/Blueprints/03_Village_Menu/Main_Village_HUD.Main_Village_HUD_C"))
  (bind _output_get (set `self.MainVillageHUDRéférence` _returnvalue))
  (`UserWidget.AddToViewport` _output_get 0)
  (bind _returnvalue_2 (`|SpawnActorFromClass` "/Game/ProjectContent/Blueprints/02_ItemLinked/BP_ItemGenerator.BP_ItemGenerator_C" (`self.Spawn Transform`) "Undefined" "OverrideRootScale" null null))
  (set `self.ItemGeneratorRef` _returnvalue_2)
  (bind _foundselectedcharacter (`self.GetSelectedCharacter`))
  (`self.GenerateItemsInMarketPlace` _foundselectedcharacter)
  (bind _asbp_game_instance (cast `/Game/ProjectContent/Blueprints/00_Manager/BP_GameInstance` (`GameplayStatics.GetGameInstance`)))
  (set `self.GameInstanceRef` _asbp_game_instance)
  (`self.PlayMusic`))

(event `CloseBasementStatWidget`
  (bind _basementstatreferences (`self.BasementStatReferences`))
  ;[0.1605 1 0.05759] Basement comportements
  (if (`KismetMathLibrary.ClassIsChildOf` (`GameplayStatics.GetObjectClass` _basementstatreferences) "/Game/ProjectContent/Blueprints/03_Village_Menu/Basement_Widgets/Basement_Stats_Widget.Basement_Stats_Widget_C")
    (`Widget.RemoveFromParent` _basementstatreferences))
  (set `self.BasementStatReferences` null)
  (set `self.StatWidgetIsOpen?` false))

(event `OpenBasementWidget`
  ;[0.1605 1 0.05759] Basement comportements
  ;;[1 1 1] Basement button click
  (bind _returnvalue (`|CreateWidget` "/Game/ProjectContent/Blueprints/03_Village_Menu/Basement_Widgets/Basement_Main_Widget.Basement_Main_Widget_C" (`GameplayStatics.GetPlayerController` 0)))
  (bind _output_get (set `self.BasementHUDRéférence` _returnvalue))
  (`UserWidget.AddToViewport` _output_get 0)
  (set `self.IsBasementOpen?` true))

(event `CloseBasementWidget`
  ;[0.1605 1 0.05759] Basement comportements
  ;;[1 1 1] Close basement widget
  (`Widget.RemoveFromParent` (`self.BasementHUDRéférence`))
  (set `self.BasementHUDRéférence` null)
  (set `self.IsBasementOpen?` false)
  (if (`KismetMathLibrary.ClassIsChildOf` (`GameplayStatics.GetObjectClass` (`self.Basement inventory reference`)) "/Game/ProjectContent/Blueprints/03_Village_Menu/Basement_Widgets/Inventory/Basement_Inventory_Widget.Basement_Inventory_Widget_C")
    (`self.CloseBasementInventoryWidget`)))

(event `OpenBasementStatsWidget`
  ;[0.1605 1 0.05759] Basement comportements
  ;;[1 1 1] Basement button click
  (bind _returnvalue (`|CreateWidget` "/Game/ProjectContent/Blueprints/03_Village_Menu/Basement_Widgets/Basement_Stats_Widget.Basement_Stats_Widget_C" (`GameplayStatics.GetPlayerController` 0)))
  (bind _output_get (set `self.BasementStatReferences` _returnvalue))
  (`UserWidget.AddToViewport` _output_get 0)
  (set `self.StatWidgetIsOpen?` true))

(event `OpenBasementInventoryWidget`
  ;[0.1605 1 0.05759] Basement comportements
  ;;[1 1 1] Basement button click
  (bind _returnvalue (`|CreateWidget` "/Game/ProjectContent/Blueprints/03_Village_Menu/Basement_Widgets/Inventory/Basement_Inventory_Widget.Basement_Inventory_Widget_C" (`GameplayStatics.GetPlayerController` 0)))
  (bind _output_get (set `self.Basement inventory reference` _returnvalue))
  (`UserWidget.AddToViewport` _output_get 0)
  (set `self.InventoryIsOpen?` true))

(event `CloseChestWidget`
  ;[0.1605 1 0.05759] Basement comportements
  ;;[1 1 1] Close basement widget
  (`Widget.RemoveFromParent` (`self.ChestWidgetReference`))
  (set `self.ChestWidgetReference` null)
  (set `self.IsChestOpen ?` false))

(event `OpenChestWidget`
  ;[0.1605 1 0.05759] Basement comportements
  ;;[1 1 1] Basement button click
  (bind _returnvalue (`|CreateWidget` "/Game/ProjectContent/Blueprints/03_Village_Menu/Basement_Widgets/Chest/Basement_Chest_Widget.Basement_Chest_Widget_C" (`GameplayStatics.GetPlayerController` 0)))
  (bind _output_get (set `self.ChestWidgetReference` _returnvalue))
  (`UserWidget.AddToViewport` _output_get 0)
  (set `self.IsChestOpen ?` true))

(event `CloseBasementInventoryWidget`
  (bind _basement_inventory_reference (`self.Basement inventory reference`))
  ;[0.1605 1 0.05759] Basement comportements
  (if (`KismetMathLibrary.ClassIsChildOf` (`GameplayStatics.GetObjectClass` _basement_inventory_reference) "/Game/ProjectContent/Blueprints/03_Village_Menu/Basement_Widgets/Inventory/Basement_Inventory_Widget.Basement_Inventory_Widget_C")
    (`Widget.RemoveFromParent` _basement_inventory_reference))
  (set `self.Basement inventory reference` null)
  (set `self.InventoryIsOpen?` false))

(event `OpenForgeWidget`
  ;[1 0.1042 0.1042] Forge comportements
  ;;[1 1 1] Forge button click
  (bind _returnvalue (`|CreateWidget` "/Game/ProjectContent/Blueprints/03_Village_Menu/Forge_Widgets/Forge_Main_Widget.Forge_Main_Widget_C" (`GameplayStatics.GetPlayerController` 0)))
  (bind _output_get (set `self.ForgeHUDReference` _returnvalue))
  (`UserWidget.AddToViewport` _output_get 0)
  (set `self.IsForgeOpen?` true))

(event `CloseForgeWidget`
  ;[1 0.1042 0.1042] Forge comportements
  ;;[1 1 1] Close forge widget
  (`Widget.RemoveFromParent` (`self.ForgeHUDReference`))
  (set `self.ForgeHUDReference` null)
  (set `self.IsForgeOpen?` false)
  (bind _foundwidgets (`WidgetBlueprintLibrary.GetAllWidgetsOfClass` "/Game/ProjectContent/Blueprints/03_Village_Menu/Forge_Widgets/Equipement_In_Forge_Widget.Equipement_In_Forge_Widget_C"))
  (`Widget.RemoveFromParent` _foundwidgets))

(event `OpenMarketplaceWidget`
  ;[0.1866 0.8701 1] Marketplace comportements
  ;;[1 1 1] Marketplace button click
  (bind _returnvalue (`|CreateWidget` "/Game/ProjectContent/Blueprints/03_Village_Menu/Marketplace_Widgets/Marketplace_Main_Widget.Marketplace_Main_Widget_C" (`GameplayStatics.GetPlayerController` 0)))
  (bind _output_get (set `self.MarketplaceHUDReference` _returnvalue))
  (`UserWidget.AddToViewport` _output_get 0)
  (set `self.IsMarketplaceOpen?` true))

(event `CloseMarketplaceWidget`
  ;[0.1866 0.8701 1] Marketplace comportements
  ;;[1 1 1] Close marketplace widget
  (`Widget.RemoveFromParent` (`self.MarketplaceHUDReference`))
  (set `self.IsMarketplaceOpen?` false)
  (set `self.MarketplaceHUDReference` null))

(event `OpenBattlefieldWidget`
  ;[1 0.8029 0.4371] Battlefield comportement
  ;;[1 1 1] Battlefield button click
  (bind _returnvalue (`|CreateWidget` "/Game/ProjectContent/Blueprints/03_Village_Menu/FrontLine_Widgets/Battlefield_Main_Widget.Battlefield_Main_Widget_C" (`GameplayStatics.GetPlayerController` 0)))
  (bind _output_get (set `self.BattlefieldHUDReference` _returnvalue))
  (`UserWidget.AddToViewport` _output_get 0))

(event `CloseBattlefieldWidget`
  ;[1 0.8029 0.4371] Battlefield comportement
  ;;[1 1 1] Close battlefield widget
  (`Widget.RemoveFromParent` (`self.BattlefieldHUDReference`))
  (set `self.BattlefieldHUDReference` null))

(fn `GenerateItemsInMarketPlace`
  (params (selectedCharacter :type "/Game/ProjectContent/Blueprints/04_PlayerLinked/BP_CharacterInfo Object Reference"))
  (for _ (range (+ (`KismetMathLibrary.RandomIntegerInRange` 7 14) 1))
    (bind _generateditem (`/Game/ProjectContent/Blueprints/02_ItemLinked/BP_ItemGenerator.Generate Item` (`self.ItemGeneratorRef`) (`KismetMathLibrary.FTrunc` (`/Game/ProjectContent/Blueprints/04_PlayerLinked/BP_Attribute.AttributeValue` (`BlueprintMapLibrary.Map_Find` (`/Game/ProjectContent/Blueprints/04_PlayerLinked/BP_CharacterInfo.DictOfAttributes` selectedCharacter) "NewEnumerator14")))))
    (`KismetArrayLibrary.Array_Add` (`self.ArrayOfMarketplaceItem`) _generateditem)))

(fn `GetAttributeValueInSelectedCharacter`
  (params (`Attribute To get ` :type "/Game/ProjectContent/Blueprints/04_PlayerLinked/AttributeEnum Enum" :default "NewEnumerator0"))
  (returns (AttributeValue :type "Float (double-precision)"))
  (bind _foundselectedcharacter (`self.GetSelectedCharacter`))
  (return (`/Game/ProjectContent/Blueprints/04_PlayerLinked/BP_Attribute.AttributeValue` (`BlueprintMapLibrary.Map_Find` (`/Game/ProjectContent/Blueprints/04_PlayerLinked/BP_CharacterInfo.DictOfAttributes` _foundselectedcharacter) `Attribute To get `))))

(fn `GetCurrentRoomLevel`
  (returns (CurrentRoomLevel :type Integer))
  (bind _asbp_game_instance (cast `/Game/ProjectContent/Blueprints/00_Manager/BP_GameInstance` (`GameplayStatics.GetGameInstance`)))
  (return (`/Game/ProjectContent/Blueprints/00_Manager/BP_GameInstance.currentRoomLevel` _asbp_game_instance)))

(fn `GetSelectedCharacter`
  (returns (FoundSelectedCharacter :type "/Game/ProjectContent/Blueprints/04_PlayerLinked/BP_CharacterInfo Object Reference"))
  (bind _asbp_game_instance (cast `/Game/ProjectContent/Blueprints/00_Manager/BP_GameInstance` (`GameplayStatics.GetGameInstance`)))
  (return (`/Game/ProjectContent/Blueprints/00_Manager/BP_GameInstance.SelectedCharacter` _asbp_game_instance)))

(fn `UserConstructionScript`)