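; BP_ItemActor is the visual actor for an item, showing a mesh and particle effect that match its ReferencedItem.
; On BeginPlay it checks whether the item class derives from BP_GoldCoin, BP_Scroll or neither, then enables the gold, scroll or generic mesh and particle system while hiding the other two.
; The item's rarity then picks color, particle count and speed, which feed the generic item particle system as parameters.
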(event `self.ReceiveBeginPlay`
  (bind _referenced_item (`self.Referenced Item`))
  (bind _itemparticlesystem (`self.ItemParticleSystem`))
  (`self.Set VFXFrom Referenced Item Class` _referenced_item)
  (`self.SetParticleInfoFromRarity` (`/Game/ProjectContent/Blueprints/02_ItemLinked/ItemHierarchy/BP_Item.ItemRarity` _referenced_item))
  (`FXSystemComponent.SetColorParameter` _itemparticlesystem "PSColor" (`self.SelectedColor`))
  (`FXSystemComponent.SetFloatParameter` _itemparticlesystem "PSNumber" (`self.SelectedNumber`))
  (`FXSystemComponent.SetFloatParameter` _itemparticlesystem "PSspeed" (`self.SelectedSpeed`)))

(fn `Set VFXFrom Referenced Item Class`
  (params (ReferencedItem :type "/Game/ProjectContent/Blueprints/02_ItemLinked/ItemHierarchy/BP_Item Object Reference (by ref)"))
  (bind _returnvalue (`GameplayStatics.GetObjectClass` ReferencedItem))
  (bind _scrollmesh (`self.ScrollMesh`))
  (bind _itemappearancemesh (`self.ItemAppearanceMesh`))
  (bind _goldmesh (`self.GoldMesh`))
  (bind _goldparticlesystem (`self.GoldParticleSystem`))
  (bind _scrollparticlesystem (`self.ScrollParticleSystem`))
  (bind _itemparticlesystem (`self.ItemParticleSystem`))
  (if (`KismetMathLibrary.ClassIsChildOf` _returnvalue "/Game/ProjectContent/Blueprints/02_ItemLinked/ItemHierarchy/BP_GoldCoin.BP_GoldCoin_C")
    ;[1 1 1] Comment
    (`self.VFXActivation` _itemparticlesystem _scrollparticlesystem _goldparticlesystem)
    (`self.MeshActivation` _scrollmesh _itemappearancemesh _goldmesh)
    (elif (`KismetMathLibrary.ClassIsChildOf` _returnvalue "/Game/ProjectContent/Blueprints/02_ItemLinked/ItemHierarchy/BP_Scroll.BP_Scroll_C")
      (`self.VFXActivation` _itemparticlesystem _goldparticlesystem _scrollparticlesystem)
      (`self.MeshActivation` _itemappearancemesh _goldmesh _scrollmesh)
      (else
        (`self.VFXActivation` _scrollparticlesystem _goldparticlesystem _itemparticlesystem)
        (`self.MeshActivation` _goldmesh _scrollmesh _itemappearancemesh)))))

(fn `SetParticleInfoFromRarity`
  (params (Selection :type "/Game/ProjectContent/Blueprints/02_ItemLinked/ItemHierarchy/RarityEnum Enum" :default "NewEnumerator0"))
  (switch `/Game/ProjectContent/Blueprints/02_ItemLinked/ItemHierarchy/RarityEnum` Selection
    (:`NewEnumerator0`
      (set `self.SelectedColor` (struct :`R` 1.0 :`G` 1.0 :`B` 1.0 :`A` 1.0))
      (set `self.SelectedNumber` 0.5)
      (set `self.SelectedSpeed` 90.0))
    (:`NewEnumerator1`
      (set `self.SelectedColor` (struct :`G` 0.028986 :`B` 1.0 :`A` 1.0))
      (set `self.SelectedNumber` 3.0)
      (set `self.SelectedSpeed` 110.0))
    (:`NewEnumerator2`
      (set `self.SelectedColor` (struct :`R` 1.0 :`G` 0.94755 :`A` 1.0))
      (set `self.SelectedNumber` 6.0)
      (set `self.SelectedSpeed` 125.0))
    (:`NewEnumerator3`
      (set `self.SelectedColor` (struct :`R` 1.0 :`G` 0.326965 :`A` 1.0))
      (set `self.SelectedNumber` 11.0)
      (set `self.SelectedSpeed` 150.0))))

(fn `UserConstructionScript`)