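; BP_PickUpGoldNumber is a floating world-space text actor that shows the amount of gold gained from a pickup.
; On BeginPlay it colors and sizes its text render component and formats it as "+ N Gold" from the GoldValue variable.
; A timeline then moves the text along Z every update, and the actor destroys itself when the timeline finishes.
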(event `self.ReceiveBeginPlay`
  (set `self.Value` (struct :`R` 180.0 :`G` 4.99997 :`A` 1.0))
  (`TextRenderComponent.SetTextRenderColor` (`self.GoldValueDisplayer`) (`KismetMathLibrary.Conv_LinearColorToColor` (`self.Value`)))
  (`TextRenderComponent.SetWorldSize` (`self.GoldValueDisplayer`) 60.0)
  (`TextRenderComponent.K2_SetText` (`self.GoldValueDisplayer`) (`|FormatText` "+ {GoldValue} Gold" (`self.GoldValue`)))
  (bind (_direction _aaa) (`Timeline|Text Mouvement`)
    (:`Update`
      (`SceneComponent.K2_AddRelativeLocation` (`self.GoldValueDisplayer`) (`KismetMathLibrary.MakeVector` 0.0 0.0 _aaa) false false))
    (:`Finished`
      (`self.K2_DestroyActor`))))

(fn `UserConstructionScript`)