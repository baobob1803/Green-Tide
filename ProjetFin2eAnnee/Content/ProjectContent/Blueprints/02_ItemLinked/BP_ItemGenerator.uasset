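; BP_ItemGenerator creates randomized RPG loot and enemy drops, and adds an item-generation button widget on BeginPlay.
; GenerateItem picks a class, level and rarity, constructs the item object, adds weapon or clothing attributes and traits, then composes its name from them.
; EnemyLootingProcedure uses the character's Magic Find and Gold Find for item, Scroll of Cowardice and gold drops, spawning each as a BP_ItemActor referencing the data object.
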(event `self.ReceiveBeginPlay`
  (bind _returnvalue (`|CreateWidget` "/Game/ProjectContent/Blueprints/02_ItemLinked/BP_ItemGenerationButton.BP_ItemGenerationButton_C"))
  (`UserWidget.AddToViewport` _returnvalue 0))

(fn `ConstructItem`
  (params (`Item Class Reference` :type "/Game/ProjectContent/Blueprints/02_ItemLinked/ItemHierarchy/BP_Item Class Reference") (Level :type Integer) (Rarity :type "/Game/ProjectContent/Blueprints/02_ItemLinked/ItemHierarchy/RarityEnum Enum" :default "NewEnumerator0"))
  (`|GenericCreateObject` `Item Class Reference` self Level Rarity))

(fn `DefineItemLevel`
  (params (`Dead Enemy Level` :type Integer))
  (returns (`Item Actual Level` :type Integer))
  (locals (FoundItemLevel :type Integer :default 0))
  (bind _output_get (set `local.FoundItemLevel` (+ `Dead Enemy Level` (`KismetMathLibrary.RandomIntegerInRange` -3 3))))
  (return (`KismetMathLibrary.Clamp` _output_get 1 100)))

(fn `DefineItemRarity`
  (returns (DefinedRarity :type "/Game/ProjectContent/Blueprints/02_ItemLinked/ItemHierarchy/RarityEnum Enum"))
  (locals (FoundRarity :type "/Game/ProjectContent/Blueprints/02_ItemLinked/ItemHierarchy/RarityEnum Enum"))
  (bind _returnvalue (`KismetMathLibrary.RandomIntegerInRange` 1 100))
  (if (< _returnvalue 5)
    (set `local.FoundRarity` "NewEnumerator3")
    (return (`local.FoundRarity`))
    (elif (< _returnvalue 15)
      (set `local.FoundRarity` "NewEnumerator2")
      (return (`local.FoundRarity`))
      (elif (< _returnvalue 35)
        (set `local.FoundRarity` "NewEnumerator1")
        (return (`local.FoundRarity`))
        (elif (< _returnvalue 100)
          (set `local.FoundRarity` "NewEnumerator0")
          (return (`local.FoundRarity`))
          (else
            (`KismetSystemLibrary.PrintString` "Bah dégage alors")))))))

(fn `Enemy Looting Procedure`
  (params (DeadEnemyTransform :type "Transform Structure") (DeadEnemyLevel :type Integer) (CurrentCharacter :type "/Game/ProjectContent/Blueprints/04_PlayerLinked/BP_CharacterInfo Object Reference"))
  (bind _dictofattributes (`/Game/ProjectContent/Blueprints/04_PlayerLinked/BP_CharacterInfo.DictOfAttributes` CurrentCharacter))
  (bind _attributevalue (`/Game/ProjectContent/Blueprints/04_PlayerLinked/BP_Attribute.AttributeValue` (`BlueprintMapLibrary.Map_Find` _dictofattributes "NewEnumerator10")))
  (bind _attributevalue_2 (`/Game/ProjectContent/Blueprints/04_PlayerLinked/BP_Attribute.AttributeValue` (`BlueprintMapLibrary.Map_Find` _dictofattributes "NewEnumerator9")))
  ;[0.7075 1 0] Should an Item Be Spawned ?
  (if (`KismetMathLibrary.InRange_FloatFloat` (* 0.1 _attributevalue_2) 0.0 10.0)
    (`self.GenerateItemFromEnemy` DeadEnemyTransform DeadEnemyLevel))
  ;[1 0.6396 0] Should A Scroll of Cowardice be spawned ?
  (if (`KismetMathLibrary.InRange_FloatFloat` (* 0.0 _attributevalue_2) 5.0 10.0)
    (`self.GenerateScrollFromEnemy` DeadEnemyTransform))
  ;[1 0.09872 0] Should Gold coins be spawned ?
  (if (`KismetMathLibrary.InRange_FloatFloat` (* 1.0 _attributevalue) 5.0 12.0)
    (`self.GenerateGoldFromEnemy` DeadEnemyTransform _attributevalue DeadEnemyLevel)))

(fn `Generate Item`
  (params (`Dead Enemy Level or Room Level` :type Integer))
  (returns (GeneratedItem :type "/Game/ProjectContent/Blueprints/02_ItemLinked/ItemHierarchy/BP_Item Object Reference"))
  (locals (NewLocalVar_3 :type String :default "RarityDenomination"))
  (bind _currentitem (`self.CurrentItem`))
  ;[0.8717 0.3181 1] Item Initial Construction from parameters
  (bind _found_class (`self.GetRandomItemClassToSpawn`))
  (bind _item_actual_level (`self.DefineItemLevel` `Dead Enemy Level or Room Level`))
  (bind _definedrarity (`self.DefineItemRarity`))
  (bind _asbp_game_instance (cast `/Game/ProjectContent/Blueprints/00_Manager/BP_GameInstance` (`GameplayStatics.GetGameInstance`)))
  (bind _returnvalue (`|GenericCreateObject` _found_class _asbp_game_instance _item_actual_level _definedrarity))
  (set `self.CurrentItem` _returnvalue)
  ;[0.001249 1 0.4999] Items gets attributes and traits considering its class
  (bind (_asbp_weapon _isitemweapon) (`self.Get Item As Weapon` (`self.CurrentItem`)))
  (if _isitemweapon
    (`self.HandleWeapon`)
    (bind _newparam (`self.SetItemName` :!label _label))
    ;[0.7874 0 1] DEBUG
    (set `/Game/ProjectContent/Blueprints/02_ItemLinked/ItemHierarchy/BP_Item.ItemName` _newparam _currentitem)
    (return _currentitem)
    (else
      (bind (_asbp_clothe _isitemclothe) (`self.Get Item As Clothe` (`self.CurrentItem`)))
      (if _isitemclothe
        (`self.HandleClothe` _asbp_clothe)
        (goto _label)))))

(fn `GenerateGoldFromEnemy`
  (params (DeadEnnemyTransform :type "Transform Structure") (PlayerGoldFind :type "Float (double-precision)") (DeadEnemyLevel :type Integer))
  (bind _returnvalue (`|GenericCreateObject` "/Game/ProjectContent/Blueprints/04_PlayerLinked/BP_Attribute.BP_Attribute_C" self "NewEnumerator20" (* (* (* PlayerGoldFind PlayerGoldFind) 0.1) (* (`KismetMathLibrary.Conv_IntToDouble` DeadEnemyLevel) 100.0))))
  (bind _returnvalue_2 (`|GenericCreateObject` "/Game/ProjectContent/Blueprints/02_ItemLinked/ItemHierarchy/BP_GoldCoin.BP_GoldCoin_C" self _returnvalue))
  (`|SpawnActorFromClass` "/Game/ProjectContent/Blueprints/02_ItemLinked/BP_ItemActor.BP_ItemActor_C" DeadEnnemyTransform "AdjustIfPossibleButAlwaysSpawn" "OverrideRootScale" null _returnvalue_2 null))

(fn `GenerateItemFromEnemy`
  (params (DeadEnemyTransform :type "Transform Structure") (`DeadEnemy Level` :type Integer))
  (bind _generateditem (`self.Generate Item` `DeadEnemy Level`))
  (`|SpawnActorFromClass` "/Game/ProjectContent/Blueprints/02_ItemLinked/BP_ItemActor.BP_ItemActor_C" DeadEnemyTransform "AdjustIfPossibleButAlwaysSpawn" "OverrideRootScale" null _generateditem null))

(fn `GenerateScrollFromEnemy`
  (params (DeadEnemyTransform :type "Transform Structure"))
  (bind _returnvalue (`|GenericCreateObject` "/Game/ProjectContent/Blueprints/02_ItemLinked/ItemHierarchy/BP_Scroll.BP_Scroll_C" self 1 1 "NewEnumerator2"))
  (`|SpawnActorFromClass` "/Game/ProjectContent/Blueprints/02_ItemLinked/BP_ItemActor.BP_ItemActor_C" DeadEnemyTransform "AdjustIfPossibleButAlwaysSpawn" "OverrideRootScale" null _returnvalue null))

(fn `Get Item As Clothe`
  (params (CurrentEquipement :type "/Game/ProjectContent/Blueprints/02_ItemLinked/ItemHierarchy/BP_Item Object Reference (by ref)"))
  (returns (`AsBP Clothe` :type "/Game/ProjectContent/Blueprints/02_ItemLinked/ItemHierarchy/BP_Clothe Object Reference") (IsItemClothe :type Boolean))
  (locals (ItemIsClothe :type Boolean))
  (if (`KismetMathLibrary.ClassIsChildOf` (`GameplayStatics.GetObjectClass` CurrentEquipement) "/Game/ProjectContent/Blueprints/02_ItemLinked/ItemHierarchy/BP_Clothe.BP_Clothe_C")
    (bind _asbp_clothe (cast `/Game/ProjectContent/Blueprints/02_ItemLinked/ItemHierarchy/BP_Clothe` CurrentEquipement))
    (set `local.ItemIsClothe` true)
    (else
      (set `local.ItemIsClothe` false)))
  (return _asbp_clothe (`local.ItemIsClothe`)))

(fn `Get Item As Misc`
  (params (CurrentEquipement :type "/Game/ProjectContent/Blueprints/02_ItemLinked/ItemHierarchy/BP_Item Object Reference (by ref)"))
  (returns (IsItemMisc :type Boolean) (`AsBP Misc` :type "/Game/ProjectContent/Blueprints/02_ItemLinked/ItemHierarchy/BP_Misc Object Reference"))
  (locals (ItemIsMisc :type Boolean))
  (if (`KismetMathLibrary.ClassIsChildOf` (`GameplayStatics.GetObjectClass` CurrentEquipement) "/Game/ProjectContent/Blueprints/02_ItemLinked/ItemHierarchy/BP_Misc.BP_Misc_C")
    (bind _asbp_misc (cast `/Game/ProjectContent/Blueprints/02_ItemLinked/ItemHierarchy/BP_Misc` CurrentEquipement))
    (set `local.ItemIsMisc` true)
    (else
      (set `local.ItemIsMisc` false)))
  (return (`local.ItemIsMisc`) _asbp_misc))

(fn `Get Item As Weapon`
  (params (CurrentEquipement :type "/Game/ProjectContent/Blueprints/02_ItemLinked/ItemHierarchy/BP_Item Object Reference (by ref)"))
  (returns (`AsBP Weapon` :type "/Game/ProjectContent/Blueprints/02_ItemLinked/ItemHierarchy/BP_Weapon Object Reference") (IsItemWeapon :type Boolean))
  (locals (ItemIsWeapon :type Boolean))
  (if (`KismetMathLibrary.ClassIsChildOf` (`GameplayStatics.GetObjectClass` CurrentEquipement) "/Game/ProjectContent/Blueprints/02_ItemLinked/ItemHierarchy/BP_Weapon.BP_Weapon_C")
    (bind _asbp_weapon (cast `/Game/ProjectContent/Blueprints/02_ItemLinked/ItemHierarchy/BP_Weapon` CurrentEquipement))
    (set `local.ItemIsWeapon` true)
    (else
      (set `local.ItemIsWeapon` false)))
  (return _asbp_weapon (`local.ItemIsWeapon`)))

(fn `GetClotheTraitName`
  (params (CurrentItem :type "/Game/ProjectContent/Blueprints/02_ItemLinked/ItemHierarchy/BP_Item Object Reference (by ref)"))
  (returns (FoundName :type String))
  (locals (NewLocalVar_0 :type String))
  (bind _asbp_clothe (cast `/Game/ProjectContent/Blueprints/02_ItemLinked/ItemHierarchy/BP_Clothe` CurrentItem))
  (for _array_element (`/Game/ProjectContent/Blueprints/02_ItemLinked/ItemHierarchy/BP_Clothe.ArrayOfClotheTraits` _asbp_clothe)
    (set `local.NewLocalVar_0` (`|GetEnumeratorNameAsString` (`/Game/ProjectContent/Blueprints/02_ItemLinked/ItemTraitsHierarchy/BP_ItemTrait.Name` _array_element))))
  (return (`local.NewLocalVar_0`)))

(fn `GetItemRarityTraitName`
  (returns (FoundRarityTraitName :type String))
  (locals (FoundName :type String))
  (for _array_element (`/Game/ProjectContent/Blueprints/02_ItemLinked/ItemHierarchy/BP_Item.RarityTraitArray` (`self.CurrentItem`))
    (set `local.FoundName` (`|GetEnumeratorNameAsString` (`/Game/ProjectContent/Blueprints/02_ItemLinked/ItemTraitsHierarchy/BP_ItemTrait.Name` _array_element))))
  (return (`local.FoundName`)))

(fn `GetRandomItemClassToSpawn`
  (returns (`Found Class` :type "/Game/ProjectContent/Blueprints/02_ItemLinked/ItemHierarchy/BP_Item Class Reference"))
  (bind _output_get (set `self.GeneratedItemClass` (`KismetArrayLibrary.Array_Random` (`self.ArrayOfAllItemClasses`))))
  (return _output_get))

(fn `GetRightDictOfRarityTraitByItemRarity`
  (returns (RightDict :type "Map of /Game/ProjectContent/Blueprints/02_ItemLinked/ItemHierarchy/TraitEnum Enum to /Game/ProjectContent/Blueprints/02_ItemLinked/RarityRawDataStruct Structure"))
  (locals (FoundDict :type "Map of /Game/ProjectContent/Blueprints/02_ItemLinked/ItemHierarchy/TraitEnum Enum to /Game/ProjectContent/Blueprints/02_ItemLinked/RarityRawDataStruct Structure"))
  (switch `/Game/ProjectContent/Blueprints/02_ItemLinked/ItemHierarchy/RarityEnum` (`/Game/ProjectContent/Blueprints/02_ItemLinked/ItemHierarchy/BP_Item.ItemRarity` (`self.CurrentItem`))
    (:`NewEnumerator0`
      (set `local.FoundDict` (`self.DictOfFrequentTraitStruct`)))
    (:`NewEnumerator1`
      (set `local.FoundDict` (`self.DictOfUncommonTraitStruct`)))
    (:`NewEnumerator2`
      (set `local.FoundDict` (`self.DictOfRareTraitStruct`)))
    (:`NewEnumerator3`
      (set `local.FoundDict` (`self.DictOfLegendaryTraitStruct`))))
  (return (`local.FoundDict`)))

(fn `GetRightTraitNameByItemType`
  (params (Array :type "Array of /Game/ProjectContent/Blueprints/02_ItemLinked/ItemTraitsHierarchy/BP_ItemTrait Object Reference") (NewParam :type "/Game/ProjectContent/Blueprints/02_ItemLinked/ItemTraitsHierarchy/BP_ItemTrait Class Reference"))
  (returns (Output_Get :type String))
  (locals (ItemSubTypeName :type String) (ClassOfTraitToLookFor :type "/Game/ProjectContent/Blueprints/02_ItemLinked/ItemTraitsHierarchy/BP_ClotheTrait Class Reference"))
  (for _array_element Array
    (if (`KismetMathLibrary.ClassIsChildOf` (`GameplayStatics.GetObjectClass` _array_element) "/Game/ProjectContent/Blueprints/02_ItemLinked/ItemTraitsHierarchy/BP_WeaponTrait.BP_WeaponTrait_C")
      (bind _output_get (set `local.ItemSubTypeName` (`|GetEnumeratorNameAsString` (`/Game/ProjectContent/Blueprints/02_ItemLinked/ItemTraitsHierarchy/BP_ItemTrait.Name` _array_element)))))))

(fn `GetWeaponTraitName`
  (params (ClassToLookFor :type "/Game/ProjectContent/Blueprints/02_ItemLinked/ItemTraitsHierarchy/BP_ItemTrait Class Reference") (CurrentItem :type "/Game/ProjectContent/Blueprints/02_ItemLinked/ItemHierarchy/BP_Item Object Reference (by ref)"))
  (returns (Found :type String))
  (locals (FoundName :type String))
  (bind _asbp_weapon (cast `/Game/ProjectContent/Blueprints/02_ItemLinked/ItemHierarchy/BP_Weapon` CurrentItem))
  (for _array_element (`/Game/ProjectContent/Blueprints/02_ItemLinked/ItemHierarchy/BP_Weapon.ArrayOfWeaponTraits` _asbp_weapon)
    (set `local.FoundName` (`|GetEnumeratorNameAsString` (`/Game/ProjectContent/Blueprints/02_ItemLinked/ItemTraitsHierarchy/BP_ItemTrait.Name` _array_element))))
  (return (`local.FoundName`)))

(fn `HandleArmoredClothe`
  (params (CurrentClothe :type "/Game/ProjectContent/Blueprints/02_ItemLinked/ItemHierarchy/Clothes/BP_ArmoredClothe Object Reference (by ref)"))
  (locals (CurrentArmoredClothe :type "Object Object Reference"))
  (bind _returnvalue (`|GenericCreateObject` "/Game/ProjectContent/Blueprints/04_PlayerLinked/BP_Attribute.BP_Attribute_C" CurrentClothe "NewEnumerator6" (`KismetMathLibrary.Conv_IntToDouble` (* (`/Game/ProjectContent/Blueprints/02_ItemLinked/ItemHierarchy/BP_Item.ItemLevel` CurrentClothe) 10))))
  (`BlueprintMapLibrary.Map_Add` (`/Game/ProjectContent/Blueprints/02_ItemLinked/ItemHierarchy/BP_Item.DictOfAttributes` CurrentClothe) (`/Game/ProjectContent/Blueprints/04_PlayerLinked/BP_Attribute.Name` _returnvalue) _returnvalue)
  (return))

(fn `HandleClothe`
  (params (CurrentClothe :type "/Game/ProjectContent/Blueprints/02_ItemLinked/ItemHierarchy/BP_Clothe Object Reference (by ref)"))
  (locals (RarityMultiplier :type "Float (double-precision)") (NewLocalVar_2 :type Integer :default 0))
  (`self.InitializeClotheAttributes` CurrentClothe)
  (`self.InititializeRandomClotheTrait` CurrentClothe)
  (bind _rightdict (`self.GetRightDictOfRarityTraitByItemRarity`))
  (`self.IntitializeRandomRarityTrait` _rightdict)
  (`self.IsClotheArmored` CurrentClothe))

(fn `HandleNonArmoredClothe`
  (params (`Current Unarmored Clothe` :type "/Game/ProjectContent/Blueprints/02_ItemLinked/ItemHierarchy/Clothes/BP_UnarmoredClothe Object Reference (by ref)"))
  (locals (CurrentUnarmoredClothe :type "/Game/ProjectContent/Blueprints/02_ItemLinked/ItemHierarchy/Clothes/UnarmoredClothes/BP_UnarmoredClothe_Abstract Object Reference"))
  (bind _dictofattributes (`/Game/ProjectContent/Blueprints/02_ItemLinked/ItemHierarchy/BP_Item.DictOfAttributes` `Current Unarmored Clothe`))
  (bind _value (`BlueprintMapLibrary.Map_Find` _dictofattributes "NewEnumerator0"))
  (bind _value_2 (`BlueprintMapLibrary.Map_Find` _dictofattributes "NewEnumerator1"))
  (set `/Game/ProjectContent/Blueprints/04_PlayerLinked/BP_Attribute.AttributeValue` (/ (`/Game/ProjectContent/Blueprints/04_PlayerLinked/BP_Attribute.AttributeValue` _value) 2.0) _value)
  (set `/Game/ProjectContent/Blueprints/04_PlayerLinked/BP_Attribute.AttributeValue` (/ (`/Game/ProjectContent/Blueprints/04_PlayerLinked/BP_Attribute.AttributeValue` _value_2) 2.0) _value_2)
  (bind _returnvalue (`|GenericCreateObject` "/Game/ProjectContent/Blueprints/04_PlayerLinked/BP_Attribute.BP_Attribute_C" `Current Unarmored Clothe` "NewEnumerator3" (`KismetMathLibrary.Conv_IntToDouble` (/ (`/Game/ProjectContent/Blueprints/02_ItemLinked/ItemHierarchy/BP_Item.ItemLevel` `Current Unarmored Clothe`) (`KismetMathLibrary.RandomIntegerInRange` 10 20)))))
  (`BlueprintMapLibrary.Map_Add` _dictofattributes (`/Game/ProjectContent/Blueprints/04_PlayerLinked/BP_Attribute.Name` _returnvalue) _returnvalue)
  (return))

(fn `HandleOneHandedWeapon`
  (params (CurrentWeapon :type "/Game/ProjectContent/Blueprints/02_ItemLinked/ItemHierarchy/BP_Weapon Object Reference (by ref)"))
  (bind _asbp_one_handed_weapon (cast `/Game/ProjectContent/Blueprints/02_ItemLinked/ItemHierarchy/Weapons/BP_OneHandedWeapon` CurrentWeapon))
  (`|ExecutionSequence`
    (:`then_0`
      (bind _dictofattributes (`/Game/ProjectContent/Blueprints/02_ItemLinked/ItemHierarchy/BP_Item.DictOfAttributes` _asbp_one_handed_weapon))
      (bind _value (`BlueprintMapLibrary.Map_Find` _dictofattributes "NewEnumerator16"))
      (set `/Game/ProjectContent/Blueprints/04_PlayerLinked/BP_Attribute.AttributeValue` (/ (`/Game/ProjectContent/Blueprints/04_PlayerLinked/BP_Attribute.AttributeValue` _value) 2.0) _value))
    (:`then_1`
      (bind _value_2 (`BlueprintMapLibrary.Map_Find` _dictofattributes "NewEnumerator15"))
      (set `/Game/ProjectContent/Blueprints/04_PlayerLinked/BP_Attribute.AttributeValue` (/ (`/Game/ProjectContent/Blueprints/04_PlayerLinked/BP_Attribute.AttributeValue` _value_2) 2.0) _value_2))
    (:`then_2`
      (bind _returnvalue (`|GenericCreateObject` "/Game/ProjectContent/Blueprints/04_PlayerLinked/BP_Attribute.BP_Attribute_C" CurrentWeapon "NewEnumerator4" (* (/ (`KismetMathLibrary.Conv_IntToDouble` (`/Game/ProjectContent/Blueprints/02_ItemLinked/ItemHierarchy/BP_Item.ItemLevel` CurrentWeapon)) 100.0) 2.147)))
      (`BlueprintMapLibrary.Map_Add` (`/Game/ProjectContent/Blueprints/02_ItemLinked/ItemHierarchy/BP_Item.DictOfAttributes` CurrentWeapon) (`/Game/ProjectContent/Blueprints/04_PlayerLinked/BP_Attribute.Name` _returnvalue) _returnvalue))))

(fn `HandleTwoHandedWeapon`
  (params (CurrentWeapon :type "/Game/ProjectContent/Blueprints/02_ItemLinked/ItemHierarchy/BP_Weapon Object Reference (by ref)"))
  (locals (currentTwoHandedWeapon :type "/Game/ProjectContent/Blueprints/02_ItemLinked/ItemHierarchy/Weapons/BP_TwoHandedWeapon Object Reference"))
  (bind _asbp_two_handed_weapon (cast `/Game/ProjectContent/Blueprints/02_ItemLinked/ItemHierarchy/Weapons/BP_TwoHandedWeapon` CurrentWeapon))
  (bind _returnvalue (`|GenericCreateObject` "/Game/ProjectContent/Blueprints/04_PlayerLinked/BP_Attribute.BP_Attribute_C" CurrentWeapon "NewEnumerator5" (`KismetMathLibrary.Conv_IntToDouble` (/ (* (`/Game/ProjectContent/Blueprints/02_ItemLinked/ItemHierarchy/BP_Item.ItemLevel` _asbp_two_handed_weapon) (`KismetMathLibrary.RandomIntegerInRange` 1 5)) 10))))
  (`BlueprintMapLibrary.Map_Add` (`/Game/ProjectContent/Blueprints/02_ItemLinked/ItemHierarchy/BP_Item.DictOfAttributes` _asbp_two_handed_weapon) (`/Game/ProjectContent/Blueprints/04_PlayerLinked/BP_Attribute.Name` _returnvalue) _returnvalue))

(fn `HandleWeapon`
  (locals (RarityMultiplier :type "Float (double-precision)" :default 0.0) (NewLocalVar_0 :type "/Game/ProjectContent/Blueprints/02_ItemLinked/ItemHierarchy/RarityEnum Enum") (NewLocalVar_1 :type "/Game/ProjectContent/Blueprints/02_ItemLinked/ItemHierarchy/BP_Weapon Object Reference") (SuperTemporaryWeapon :type "/Game/ProjectContent/Blueprints/02_ItemLinked/ItemHierarchy/BP_Weapon Object Reference"))
  (bind _asbp_weapon (cast `/Game/ProjectContent/Blueprints/02_ItemLinked/ItemHierarchy/BP_Weapon` (`self.CurrentItem`)))
  (`self.InitializeWeaponAttributes` _asbp_weapon)
  (`self.InitializeRandomWeaponTraits` _asbp_weapon)
  (bind _rightdict (`self.GetRightDictOfRarityTraitByItemRarity`))
  (`self.IntitializeRandomRarityTrait` _rightdict)
  (`self.IsWeaponOneHanded` _asbp_weapon))

(fn `InitializeClotheAttributes`
  (params (self2 :type "/Game/ProjectContent/Blueprints/02_ItemLinked/ItemHierarchy/BP_Item Object Reference"))
  (bind _dictofattributes (`/Game/ProjectContent/Blueprints/02_ItemLinked/ItemHierarchy/BP_Item.DictOfAttributes` self2))
  (bind _returnvalue (* (* (`/Game/ProjectContent/Blueprints/02_ItemLinked/ItemHierarchy/BP_Item.ItemLevel` self2) (`KismetMathLibrary.RandomFloatInRange` 2.0 4.0)) 1.0))
  (bind _returnvalue_2 (`|GenericCreateObject` "/Game/ProjectContent/Blueprints/04_PlayerLinked/BP_Attribute.BP_Attribute_C" self2 "NewEnumerator1" _returnvalue))
  (`BlueprintMapLibrary.Map_Add` _dictofattributes (`/Game/ProjectContent/Blueprints/04_PlayerLinked/BP_Attribute.Name` _returnvalue_2) _returnvalue_2)
  (bind _returnvalue_3 (`|GenericCreateObject` "/Game/ProjectContent/Blueprints/04_PlayerLinked/BP_Attribute.BP_Attribute_C" self2 "NewEnumerator0" _returnvalue))
  (`BlueprintMapLibrary.Map_Add` _dictofattributes (`/Game/ProjectContent/Blueprints/04_PlayerLinked/BP_Attribute.Name` _returnvalue_3) _returnvalue_3))

(fn `InitializeRandomWeaponTraits`
  (params (CurrentWeapon :type "/Game/ProjectContent/Blueprints/02_ItemLinked/ItemHierarchy/BP_Weapon Object Reference (by ref)"))
  (bind _values (`BlueprintMapLibrary.Map_Values` (`self.DictOfWeaponTraitStruct`)))
  (bind _outitem (`KismetArrayLibrary.Array_Random` _values))
  (bind _returnvalue (`|GenericCreateObject` "/Game/ProjectContent/Blueprints/02_ItemLinked/ItemTraitsHierarchy/BP_WeaponTrait.BP_WeaponTrait_C" CurrentWeapon (break `/Game/ProjectContent/Blueprints/02_ItemLinked/TraitRawDataStruct` _outitem) (`.InfluencedAttribute_10_C2B74AD647179EF03EF5D48A74EB81A0` (break `/Game/ProjectContent/Blueprints/02_ItemLinked/TraitRawDataStruct` _outitem)) (* (`.TraitBaseValue_11_07D0DBDD4E26F6E81BF2FAAF57FD9C39` (break `/Game/ProjectContent/Blueprints/02_ItemLinked/TraitRawDataStruct` _outitem)) (* (`.TraitMultiplier_12_77F651324F1084B84EE779BE56A7319C` (break `/Game/ProjectContent/Blueprints/02_ItemLinked/TraitRawDataStruct` _outitem)) (`KismetMathLibrary.Conv_IntToDouble` (`/Game/ProjectContent/Blueprints/02_ItemLinked/ItemHierarchy/BP_Item.ItemLevel` CurrentWeapon))))))
  (`KismetArrayLibrary.Array_Add` (`/Game/ProjectContent/Blueprints/02_ItemLinked/ItemHierarchy/BP_Weapon.ArrayOfWeaponTraits` CurrentWeapon) _returnvalue))

(fn `InitializeWeaponAttributes`
  (params (Output_Get :type "/Game/ProjectContent/Blueprints/02_ItemLinked/ItemHierarchy/BP_Weapon Object Reference (by ref)"))
  (bind _itemlevel (`/Game/ProjectContent/Blueprints/02_ItemLinked/ItemHierarchy/BP_Item.ItemLevel` Output_Get))
  (bind _dictofattributes (`/Game/ProjectContent/Blueprints/02_ItemLinked/ItemHierarchy/BP_Item.DictOfAttributes` Output_Get))
  (bind _returnvalue (`|GenericCreateObject` "/Game/ProjectContent/Blueprints/04_PlayerLinked/BP_Attribute.BP_Attribute_C" "BP_ItemGenerator" "NewEnumerator2" (* (* (`/Game/ProjectContent/Blueprints/02_ItemLinked/ItemHierarchy/BP_Item.ItemLevel` Output_Get) (`KismetMathLibrary.RandomFloatInRange` 2.0 4.0)) 1.0)))
  (`BlueprintMapLibrary.Map_Add` _dictofattributes (`/Game/ProjectContent/Blueprints/04_PlayerLinked/BP_Attribute.Name` _returnvalue) _returnvalue)
  (bind _returnvalue_2 (`|GenericCreateObject` "/Game/ProjectContent/Blueprints/04_PlayerLinked/BP_Attribute.BP_Attribute_C" "BP_ItemGenerator" "NewEnumerator15" (`KismetMathLibrary.Conv_IntToDouble` (+ (`KismetMathLibrary.RandomIntegerInRange` 5 15) _itemlevel))))
  (`BlueprintMapLibrary.Map_Add` _dictofattributes (`/Game/ProjectContent/Blueprints/04_PlayerLinked/BP_Attribute.Name` _returnvalue_2) _returnvalue_2)
  (bind _returnvalue_3 (`|GenericCreateObject` "/Game/ProjectContent/Blueprints/04_PlayerLinked/BP_Attribute.BP_Attribute_C" "BP_ItemGenerator" "NewEnumerator16" (`KismetMathLibrary.Conv_IntToDouble` (+ _itemlevel (`KismetMathLibrary.RandomIntegerInRange` 16 30)))))
  (`BlueprintMapLibrary.Map_Add` _dictofattributes (`/Game/ProjectContent/Blueprints/04_PlayerLinked/BP_Attribute.Name` _returnvalue_3) _returnvalue_3))

(fn `InititializeRandomClotheTrait`
  (params (cLOTHE :type "/Game/ProjectContent/Blueprints/02_ItemLinked/ItemHierarchy/BP_Clothe Object Reference"))
  (bind _values (`BlueprintMapLibrary.Map_Values` (`self.DictOfClothTraitStruct`)))
  (bind _outitem (`KismetArrayLibrary.Array_Random` _values))
  (bind _returnvalue (`|GenericCreateObject` "/Game/ProjectContent/Blueprints/02_ItemLinked/ItemTraitsHierarchy/BP_ClotheTrait.BP_ClotheTrait_C" cLOTHE (break `/Game/ProjectContent/Blueprints/02_ItemLinked/TraitRawDataStruct` _outitem) (`.InfluencedAttribute_10_C2B74AD647179EF03EF5D48A74EB81A0` (break `/Game/ProjectContent/Blueprints/02_ItemLinked/TraitRawDataStruct` _outitem)) (* (`.TraitBaseValue_11_07D0DBDD4E26F6E81BF2FAAF57FD9C39` (break `/Game/ProjectContent/Blueprints/02_ItemLinked/TraitRawDataStruct` _outitem)) (* (`.TraitMultiplier_12_77F651324F1084B84EE779BE56A7319C` (break `/Game/ProjectContent/Blueprints/02_ItemLinked/TraitRawDataStruct` _outitem)) (`KismetMathLibrary.Conv_IntToDouble` (`/Game/ProjectContent/Blueprints/02_ItemLinked/ItemHierarchy/BP_Item.ItemLevel` cLOTHE))))))
  (`KismetArrayLibrary.Array_Add` (`/Game/ProjectContent/Blueprints/02_ItemLinked/ItemHierarchy/BP_Clothe.ArrayOfClotheTraits` cLOTHE) _returnvalue))

(fn `IntitializeRandomRarityTrait`
  (params (DictOfRarityTrait :type "Map of /Game/ProjectContent/Blueprints/02_ItemLinked/ItemHierarchy/TraitEnum Enum to /Game/ProjectContent/Blueprints/02_ItemLinked/RarityRawDataStruct Structure"))
  (bind _currentitem (`self.CurrentItem`))
  (bind _values (`BlueprintMapLibrary.Map_Values` DictOfRarityTrait))
  (bind _outitem (`KismetArrayLibrary.Array_Random` _values))
  (bind _returnvalue (`|GenericCreateObject` "/Game/ProjectContent/Blueprints/02_ItemLinked/ItemTraitsHierarchy/BP_RarityTrait.BP_RarityTrait_C" _currentitem (`/Game/ProjectContent/Blueprints/02_ItemLinked/ItemHierarchy/BP_Item.ItemRarity` _currentitem) (break `/Game/ProjectContent/Blueprints/02_ItemLinked/RarityRawDataStruct` _outitem) (`.InfluencedTrait_7_0045294249E1522B0E2B9C9CBF796FF1` (break `/Game/ProjectContent/Blueprints/02_ItemLinked/RarityRawDataStruct` _outitem)) (* (`.BaseValue_13_B2A5809E42789F086B46E292D042974D` (break `/Game/ProjectContent/Blueprints/02_ItemLinked/RarityRawDataStruct` _outitem)) (* (`.Multiplier_15_122E609A49A39A7524E1ABA31B1D27C1` (break `/Game/ProjectContent/Blueprints/02_ItemLinked/RarityRawDataStruct` _outitem)) (`KismetMathLibrary.Conv_IntToDouble` (`/Game/ProjectContent/Blueprints/02_ItemLinked/ItemHierarchy/BP_Item.ItemLevel` _currentitem))))))
  (`KismetArrayLibrary.Array_Add` (`/Game/ProjectContent/Blueprints/02_ItemLinked/ItemHierarchy/BP_Item.RarityTraitArray` _currentitem) _returnvalue)
  (return))

(fn `IsClotheArmored`
  (params (CurrentClothe :type "/Game/ProjectContent/Blueprints/02_ItemLinked/ItemHierarchy/BP_Clothe Object Reference (by ref)"))
  (locals (`Recasted Item` :type "Object Object Reference"))
  (if (`KismetMathLibrary.ClassIsChildOf` (`GameplayStatics.GetObjectClass` CurrentClothe))
    (bind _asbp_armored_clothe (cast `/Game/ProjectContent/Blueprints/02_ItemLinked/ItemHierarchy/Clothes/BP_ArmoredClothe` CurrentClothe))
    (`self.HandleArmoredClothe` _asbp_armored_clothe)
    (else
      (bind _asbp_unarmored_clothe (cast `/Game/ProjectContent/Blueprints/02_ItemLinked/ItemHierarchy/Clothes/BP_UnarmoredClothe` CurrentClothe))
      (`self.HandleNonArmoredClothe` _asbp_unarmored_clothe)))
  (return))

(fn `IsWeaponOneHanded`
  (params (CurrentWeapon :type "/Game/ProjectContent/Blueprints/02_ItemLinked/ItemHierarchy/BP_Weapon Object Reference (by ref)"))
  (locals (`Recasted Item` :type "Object Object Reference"))
  (if (`KismetMathLibrary.ClassIsChildOf` (`GameplayStatics.GetObjectClass` CurrentWeapon) "/Game/ProjectContent/Blueprints/02_ItemLinked/ItemHierarchy/Weapons/BP_OneHandedWeapon.BP_OneHandedWeapon_C")
    (`self.HandleOneHandedWeapon` CurrentWeapon)
    (else
      (`self.HandleTwoHandedWeapon` CurrentWeapon))))

(fn `SetItemName`
  (returns (NewParam :type String))
  (locals (TraitsClassToLookFor :type "/Game/ProjectContent/Blueprints/02_ItemLinked/ItemTraitsHierarchy/BP_ItemTrait Class Reference") (TempArrayOfRarityDenomination :type "Array of String") (ItemTypeName :type String) (ItemSubTypeName :type String) (ItemRarityTraitName :type String))
  (bind _currentitem (`self.CurrentItem`))
  (bind _currentitem_2 (`self.CurrentItem`))
  (bind _returnvalue (`GameplayStatics.GetObjectClass` _currentitem))
  (bind _returnvalue_2 (`KismetSystemLibrary.GetClassDisplayName` _returnvalue))
  (if (`KismetMathLibrary.ClassIsChildOf` _returnvalue "/Game/ProjectContent/Blueprints/02_ItemLinked/ItemHierarchy/BP_Misc.BP_Misc_C")
    (set `/Game/ProjectContent/Blueprints/02_ItemLinked/ItemHierarchy/BP_Item.ItemName` "Scroll Of Cowardice" _currentitem)
    (else
      (switch `/Game/ProjectContent/Blueprints/02_ItemLinked/ItemHierarchy/RarityEnum` (`/Game/ProjectContent/Blueprints/02_ItemLinked/ItemHierarchy/BP_Item.ItemRarity` _currentitem)
        (:`NewEnumerator0`
          (set `local.TempArrayOfRarityDenomination` (`self.ArrayOfFrequentDenomination`)))
        (:`NewEnumerator1`
          (set `local.TempArrayOfRarityDenomination` (`self.ArrayOfUncommonDenomination`)))
        (:`NewEnumerator2`
          (set `local.TempArrayOfRarityDenomination` (`self.ArrayOfRareDenomination`)))
        (:`NewEnumerator3`
          (set `local.TempArrayOfRarityDenomination` (`self.ArrayOfLegendaryDenomination`))))
      (if (`KismetMathLibrary.ClassIsChildOf` _returnvalue "/Game/ProjectContent/Blueprints/02_ItemLinked/ItemHierarchy/BP_Weapon.BP_Weapon_C")
        (set `local.TraitsClassToLookFor` "/Game/ProjectContent/Blueprints/02_ItemLinked/ItemTraitsHierarchy/BP_WeaponTrait.BP_WeaponTrait_C")
        (if (`KismetStringLibrary.Contains` _returnvalue_2 "OneHanded")
          (bind _output_get (set `local.ItemTypeName` _returnvalue_2))
          (set `local.ItemTypeName` (`KismetStringLibrary.LeftChop` (`KismetStringLibrary.RightChop` _output_get 12) 2))
          (else
            (bind _output_get_2 (set `local.ItemTypeName` _returnvalue_2))
            (set `local.ItemTypeName` (`KismetStringLibrary.LeftChop` (`KismetStringLibrary.RightChop` _output_get_2 12) 2))))
        (bind _found (`self.GetWeaponTraitName` null _currentitem_2))
        (set `local.ItemSubTypeName` _found)
        (else
          (set `local.TraitsClassToLookFor` "/Game/ProjectContent/Blueprints/02_ItemLinked/ItemTraitsHierarchy/BP_ClotheTrait.BP_ClotheTrait_C")
          (if (`KismetStringLibrary.Contains` _returnvalue_2 "Unarmored")
            (bind _output_get_3 (set `local.ItemTypeName` _returnvalue_2))
            (set `local.ItemTypeName` (`KismetStringLibrary.LeftChop` (`KismetStringLibrary.RightChop` _output_get_3 12) 2))
            (else
              (bind _output_get_4 (set `local.ItemTypeName` _returnvalue_2))
              (set `local.ItemTypeName` (`KismetStringLibrary.LeftChop` (`KismetStringLibrary.RightChop` _output_get_4 10) 2))))
          (bind _foundname (`self.GetClotheTraitName` _currentitem_2))
          (set `local.ItemSubTypeName` _foundname)))
      (bind _foundraritytraitname (`self.GetItemRarityTraitName`))
      (set `local.ItemRarityTraitName` _foundraritytraitname)
      (return (`KismetStringLibrary.Concat_StrStr` (`KismetArrayLibrary.Array_Random` (`local.TempArrayOfRarityDenomination`)) " " (`local.ItemTypeName`) " Of " (`local.ItemSubTypeName`) " " (`local.ItemRarityTraitName`) " ")))))

(fn `UserConstructionScript`)