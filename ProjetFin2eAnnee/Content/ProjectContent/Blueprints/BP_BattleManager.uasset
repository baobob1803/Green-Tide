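; Battle manager actor that drives room-to-room progression and opens the battle stat and inventory screens.
; On BeginPlay it spawns an item generator, caches the player, wave manager and game instance, and increments the room streak.
; OnNextRoom updates room level, streak and HUD, notifies the player, destroys leftover items, then generates a wave after a short delay.
; Each screen request removes existing battle widgets and recreates the main widget on the requested panel.
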(event `self.ReceiveBeginPlay`
  (`self.Get Ref for ItemGenerator, Player, WaveManager & Game Instance`)
  (`/Game/ProjectContent/Blueprints/00_Manager/BP_GameInstance.Increment Room in ARow` (`self.gameinstance`)))

(event `OnNextRoom`
  (bind _gameinstance (`self.gameinstance`))
  (`/Game/ProjectContent/Blueprints/00_Manager/BP_GameInstance.UpdateRoomLevel` _gameinstance)
  (`/Game/ProjectContent/Blueprints/00_Manager/BP_GameInstance.Increment Room in ARow` _gameinstance)
  (bind _returnvalue (`GameplayStatics.GetActorOfClass` "/Game/ProjectContent/BP_Character_Master.BP_Character_Master_C"))
  (`/Game/ProjectContent/Blueprints/06_LayoutMapGeneration/CharaInfoDisplayerInCombat.Display RoomInARow Value ` (`/Game/ProjectContent/BP_Character_Master.CombatHUDRef` _returnvalue))
  (`/Game/ProjectContent/BP_Character_Master.OnNextRoom` (`self.player`))
  (`self.DestroyRemainingItemActors`)
  (`KismetSystemLibrary.Delay` 0.2)
  (`/Game/ProjectContent/Enemies/BP_RealWaveManager.GenerateWave` (`self.waveManager`) (`/Game/ProjectContent/Blueprints/00_Manager/BP_GameInstance.currentRoomLevel` (`self.gameinstance`))))

(event `Display Widget BattleStat`
  ;[0.7102 0.6878 1] Widget Displayer
  (`self.Open Inventory W/Battle Stat Widget`))

(event `Display Widget Battle Inventory`
  ;[0.7102 0.6878 1] Widget Displayer
  (`self.Open Inventory W/Battle Inventory Widget`))

(fn `DestroyRemainingItemActors`
  (bind _outactors (`GameplayStatics.GetAllActorsOfClass` "/Game/ProjectContent/Blueprints/02_ItemLinked/BP_ItemActor.BP_ItemActor_C"))
  (for _array_element _outactors
    (`self.K2_DestroyActor` _array_element))
  (`KismetSystemLibrary.PrintString` "All items have been successfully destroyed"))

(fn `Get Ref for ItemGenerator, Player, WaveManager & Game Instance`
  ;[1 1 1] Item Generator Ref
  (bind _returnvalue (`|SpawnActorFromClass` "/Game/ProjectContent/Blueprints/02_ItemLinked/BP_ItemGenerator.BP_ItemGenerator_C" (`self.Spawn Transform`) "AdjustIfPossibleButAlwaysSpawn" "OverrideRootScale" null null))
  (set `self.ItemGeneratorRef` _returnvalue)
  ;[1 1 1] Player Ref
  (bind _returnvalue_2 (`GameplayStatics.GetActorOfClass` "/Game/ProjectContent/BP_Character_Master.BP_Character_Master_C"))
  (set `self.player` _returnvalue_2)
  ;[1 1 1] Wave Manager Ref
  (bind _returnvalue_3 (`GameplayStatics.GetActorOfClass` "/Game/ProjectContent/Enemies/BP_RealWaveManager.BP_RealWaveManager_C"))
  (set `self.waveManager` _returnvalue_3)
  ;[1 1 1] Game Instance Ref
  (bind _asbp_game_instance (cast `/Game/ProjectContent/Blueprints/00_Manager/BP_GameInstance` (`GameplayStatics.GetGameInstance`))
    (:`then`
      (set `self.gameinstance` _asbp_game_instance))
    (:`CastFailed`
      (`KismetSystemLibrary.PrintString` "Failed Cast to Game INstance in BattleManager"))))

(fn `IncrementCharacterRoomInARown`
  (`/Engine/EditorBlueprintResources/StandardMacros.IncrementInt` (`/Game/ProjectContent/Blueprints/04_PlayerLinked/BP_CharacterInfo.Room Row Number` (`/Game/ProjectContent/Blueprints/00_Manager/BP_GameInstance.SelectedCharacter` (`self.gameinstance`)))))

(fn `Open Inventory W/Battle Inventory Widget`
  (bind _battlemainwidgetref (`self.BattleMainWidgetRef`))
  (bind _battlestatwidgetref (`/Game/ProjectContent/Blueprints/05_InBattleMenu/Battle_MainWidget.BattleStatWidgetRef` _battlemainwidgetref))
  (bind _battleinventorywidgetref (`/Game/ProjectContent/Blueprints/05_InBattleMenu/Battle_MainWidget.BattleInventoryWidgetRef` _battlemainwidgetref))
  (if (`KismetMathLibrary.ClassIsChildOf` (`GameplayStatics.GetObjectClass` _battlemainwidgetref) "/Game/ProjectContent/Blueprints/05_InBattleMenu/Battle_MainWidget.Battle_MainWidget_C")
    (`Widget.RemoveFromParent` _battlemainwidgetref))
  (if (`KismetMathLibrary.ClassIsChildOf` (`GameplayStatics.GetObjectClass` _battlestatwidgetref) "/Game/ProjectContent/Blueprints/05_InBattleMenu/Battle_StatWidget.Battle_StatWidget_C")
    (`Widget.RemoveFromParent` _battlestatwidgetref))
  (if (`KismetMathLibrary.ClassIsChildOf` (`GameplayStatics.GetObjectClass` _battleinventorywidgetref) "/Game/ProjectContent/Blueprints/05_InBattleMenu/Battle_InventoryWidget.Battle_InventoryWidget_C")
    (`Widget.RemoveFromParent` _battleinventorywidgetref))
  (bind _returnvalue (`|CreateWidget` "/Game/ProjectContent/Blueprints/05_InBattleMenu/Battle_MainWidget.Battle_MainWidget_C"))
  (bind _output_get (set `self.BattleMainWidgetRef` _returnvalue))
  (`UserWidget.AddToViewport` _output_get 0)
  (`/Game/ProjectContent/Blueprints/05_InBattleMenu/Battle_MainWidget.Display Battle Inventory Widget` _output_get))

(fn `Open Inventory W/Battle Stat Widget`
  (bind _battlemainwidgetref (`self.BattleMainWidgetRef`))
  (bind _battlestatwidgetref (`/Game/ProjectContent/Blueprints/05_InBattleMenu/Battle_MainWidget.BattleStatWidgetRef` _battlemainwidgetref))
  (bind _battleinventorywidgetref (`/Game/ProjectContent/Blueprints/05_InBattleMenu/Battle_MainWidget.BattleInventoryWidgetRef` _battlemainwidgetref))
  (if (`KismetMathLibrary.ClassIsChildOf` (`GameplayStatics.GetObjectClass` _battlemainwidgetref) "/Game/ProjectContent/Blueprints/05_InBattleMenu/Battle_MainWidget.Battle_MainWidget_C")
    (`Widget.RemoveFromParent` _battlemainwidgetref))
  (if (`KismetMathLibrary.ClassIsChildOf` (`GameplayStatics.GetObjectClass` _battlestatwidgetref) "/Game/ProjectContent/Blueprints/05_InBattleMenu/Battle_StatWidget.Battle_StatWidget_C")
    (`Widget.RemoveFromParent` _battlestatwidgetref))
  (if (`KismetMathLibrary.ClassIsChildOf` (`GameplayStatics.GetObjectClass` _battleinventorywidgetref) "/Game/ProjectContent/Blueprints/05_InBattleMenu/Battle_InventoryWidget.Battle_InventoryWidget_C")
    (`Widget.RemoveFromParent` _battleinventorywidgetref))
  (bind _returnvalue (`|CreateWidget` "/Game/ProjectContent/Blueprints/05_InBattleMenu/Battle_MainWidget.Battle_MainWidget_C"))
  (bind _output_get (set `self.BattleMainWidgetRef` _returnvalue))
  (`UserWidget.AddToViewport` _output_get 0)
  (`/Game/ProjectContent/Blueprints/05_InBattleMenu/Battle_MainWidget.Display Battle Stat Widget` _output_get))

(fn `UserConstructionScript`)