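; Village menu manager that creates and shows the main village HUD on BeginPlay and handles the screens for the village's locations.
; Open and close events create, store and remove widgets for the Basement, its stats panel, the Forge, Marketplace and Battlefield.
; The basement inventory close event is an empty stub.
; It also reads the selected character from BP_GameInstance at startup, but the returned value goes unused.
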(event `self.ReceiveBeginPlay`
  ;[1 1 1] Creat & reference main village HUD
  (`self.GetSelectedCharacter`)
  (bind _returnvalue (`|CreateWidget` "/Game/ProjectContent/Blueprints/02_Village_Menu/Main_Village_HUD.Main_Village_HUD_C"))
  (bind _output_get (set `self.MainVillageHUDRéférence` _returnvalue))
  (`UserWidget.AddToViewport` _output_get 0))

(event `OpenBasementWidget`
  ;[0.1605 1 0.05759] Basement comportements
  ;;[1 1 1] Basement button click
  (bind _returnvalue (`|CreateWidget` "/Game/ProjectContent/Blueprints/02_Village_Menu/Basement_Widgets/Basement_Main_Widget.Basement_Main_Widget_C" (`GameplayStatics.GetPlayerController` 0)))
  (bind _output_get (set `self.BasementHUDRéférence` _returnvalue))
  (`UserWidget.AddToViewport` _output_get 0))

(event `CloseBasementWidget`
  ;[0.1605 1 0.05759] Basement comportements
  ;;[1 1 1] Close basement widget
  (`Widget.RemoveFromParent` (`self.BasementHUDRéférence`))
  (set `self.BasementHUDRéférence` null))

(event `CloseBasementStatWidget`
  ;[0.1605 1 0.05759] Basement comportements
  ;;[1 1 1] Close basement widget
  (`Widget.RemoveFromParent` (`self.BasementStatReferences`))
  (set `self.BasementStatReferences` null))

(event `OpenBasementStatsWidget`
  ;[0.1605 1 0.05759] Basement comportements
  ;;[1 1 1] Basement button click
  (bind _returnvalue (`|CreateWidget` "/Game/ProjectContent/Blueprints/02_Village_Menu/Basement_Widgets/Basement_Stats_Widget.Basement_Stats_Widget_C" (`GameplayStatics.GetPlayerController` 0)))
  (bind _output_get (set `self.BasementStatReferences` _returnvalue))
  (`UserWidget.AddToViewport` _output_get 0))

(event `CloseBasementInventoryWidget`
  ;[0.1605 1 0.05759] Basement comportements
  ;;[1 1 1] Close basement widget
)

(event `OpenForgeWidget`
  ;[1 0.1042 0.1042] Forge comportements
  ;;[1 1 1] Forge button click
  (bind _returnvalue (`|CreateWidget` "/Game/ProjectContent/Blueprints/02_Village_Menu/Forge_Widgets/Forge_Main_Widget.Forge_Main_Widget_C" (`GameplayStatics.GetPlayerController` 0)))
  (bind _output_get (set `self.ForgeHUDReference` _returnvalue))
  (`UserWidget.AddToViewport` _output_get 0))

(event `CloseForgeWidget`
  ;[1 0.1042 0.1042] Forge comportements
  ;;[1 1 1] Close forge widget
  (`Widget.RemoveFromParent` (`self.ForgeHUDReference`))
  (set `self.ForgeHUDReference` null))

(event `OpenMarketplaceWidget`
  ;[0.1866 0.8701 1] Marketplace comportements
  ;;[1 1 1] Marketplace button click
  (bind _returnvalue (`|CreateWidget` "/Game/ProjectContent/Blueprints/02_Village_Menu/Marketplace_Widgets/Marketplace_Main_Widget.Marketplace_Main_Widget_C" (`GameplayStatics.GetPlayerController` 0)))
  (bind _output_get (set `self.MarketplaceHUDReference` _returnvalue))
  (`UserWidget.AddToViewport` _output_get 0))

(event `CloseMarketplaceWidget`
  ;[0.1866 0.8701 1] Marketplace comportements
  ;;[1 1 1] Close marketplace widget
  (`Widget.RemoveFromParent` (`self.MarketplaceHUDReference`))
  (set `self.MarketplaceHUDReference` null))

(event `OpenBattlefieldWidget`
  ;[1 0.8029 0.4371] Battlefield comportement
  ;;[1 1 1] Battlefield button click
  (bind _returnvalue (`|CreateWidget` "/Game/ProjectContent/Blueprints/02_Village_Menu/Battlefield_Widgets/Battlefield_Main_Widget.Battlefield_Main_Widget_C" (`GameplayStatics.GetPlayerController` 0)))
  (bind _output_get (set `self.BattlefieldHUDReference` _returnvalue))
  (`UserWidget.AddToViewport` _output_get 0))

(event `CloseBattlefieldWidget`
  ;[1 0.8029 0.4371] Battlefield comportement
  ;;[1 1 1] Close battlefield widget
  (`Widget.RemoveFromParent` (`self.BattlefieldHUDReference`))
  (set `self.BattlefieldHUDReference` null))

(fn `GetSelectedCharacter`
  (returns (FoundSelectedCharacter :type "/Game/ProjectContent/Blueprints/PlayerLinked/BP_CharacterInfo Object Reference"))
  (bind _asbp_game_instance (cast `/Game/ProjectContent/Blueprints/00_Manager/BP_GameInstance` (`GameplayStatics.GetGameInstance`)))
  (return (`/Game/ProjectContent/Blueprints/00_Manager/BP_GameInstance.SelectedCharacter` _asbp_game_instance)))

(fn `UserConstructionScript`)