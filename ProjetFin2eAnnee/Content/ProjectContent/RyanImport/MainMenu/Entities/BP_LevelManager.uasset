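; Main menu manager actor that opens the menu widgets and handles player profile creation.
; On BeginPlay it caches the game instance's profile array and shows the main menu; button events add or remove the profile and creation widgets.
; Confirming creation rejects empty or duplicate names and a full list.
; Valid profiles spawn as BP_PlayerProfile actors, take their array index as ID, and the array is written back to the game instance.
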(event `self.ReceiveBeginPlay`
  ;[1 1 1] Comment
  (bind _asbp_game_instance (cast `/Game/MainMenu/BP_GameInstance` (`GameplayStatics.GetGameInstance`)))
  (bind _output_get (set `self.GameInstanceReference` _asbp_game_instance))
  (set `self.LocalArrayOfPlayerProfiles` (`/Game/MainMenu/BP_GameInstance.ArrayOfPlayerProfile` _output_get))
  ;[1 1 1] Creating and referencing Main Menu Widget
  (bind _returnvalue (`|CreateWidget` "/Game/MainMenu/UI_MainMenu_BP.UI_MainMenu_BP_C" (`GameplayStatics.GetPlayerController` 0)))
  (bind _output_get_2 (set `self.MainMenuReference` _returnvalue))
  (`UserWidget.AddToViewport` _output_get_2 0))

(event `BackButtonClicked(ProfileMenu)`
  ;[1 0.7581 0.1451 1 36] Profile Menu Linked Events
  ;;[0.4167 0.3531 0.1156] Back From Profile Menu
  (`Widget.RemoveFromParent` (`self.ProfileMenuReference`)))

(event `ProfileMenuButtonClicked`
  ;[1 0.7581 0.1451 1 36] Profile Menu Linked Events
  ;;[0.151 0.1425 0.05282] Profile Button Click
  (bind _returnvalue (`|CreateWidget` "/Game/MainMenu/CreateProfileMenu/UI_ProfileMenu.UI_ProfileMenu_C" (`GameplayStatics.GetPlayerController` 0)))
  (bind _output_get (set `self.ProfileMenuReference` _returnvalue))
  (`UserWidget.AddToViewport` _output_get 0))

(event `CreateNewProfileButtonTapped`
  ;[1 0.7581 0.1451 1 36] Profile Menu Linked Events
  ;;[1 1 1] Comment
  (bind _returnvalue (`|CreateWidget` "/Game/MainMenu/CreateProfileMenu/UI_CreateNewProfileMenu.UI_CreateNewProfileMenu_C" (`GameplayStatics.GetPlayerController` 0)))
  (bind _output_get (set `self.CreateNewProfileMenuReference` _returnvalue))
  (`UserWidget.AddToViewport` _output_get 0))

(event `ConfirmProfileCreationClicked`
  (bind _localarrayofplayerprofiles (`self.LocalArrayOfPlayerProfiles`))
  (bind _lastcreatedplayerprofile (`self.LastCreatedPlayerProfile`))
  ;[1 1 1] Comment
  (if (`KismetTextLibrary.TextIsEmpty` (`KismetTextLibrary.Conv_StringToText` (`/Game/MainMenu/CreateProfileMenu/UI_CreateNewProfileMenu.CurrentProfileName` (`self.CreateNewProfileMenuReference`))))
    (`KismetSystemLibrary.PrintString` "Cannot Submit an empty name")
    (`KismetSystemLibrary.CollectGarbage`)
    (else
      ;;[1 1 1] Profile List Full - Check
      (if (== (`KismetArrayLibrary.Array_Length` (`self.LocalArrayOfPlayerProfiles`)) 5)
        (`KismetSystemLibrary.PrintString` "Cannot create more than 5 profiles")
        (`KismetSystemLibrary.CollectGarbage`)
        (else
          ;;[1 1 1] ProfileNameAlreadyExists - Check
          (for _array_element (`self.LocalArrayOfPlayerProfiles`)
            (if (`KismetStringLibrary.EqualEqual_StrStr` (`/Game/MainMenu/Entities/BP_PlayerProfile.ProfileName` _array_element) (`/Game/MainMenu/CreateProfileMenu/UI_CreateNewProfileMenu.CurrentProfileName` (`self.CreateNewProfileMenuReference`)))
              (`KismetSystemLibrary.PrintString` "A profile with thime name already exists")
              (set `self.SameNameFound` true)))
          (if (`self.SameNameFound`)
            (`KismetSystemLibrary.PrintString` "Profile Did not spawn")
            (`KismetSystemLibrary.CollectGarbage`)
            (else
              ;;[1 1 1] GeneratingNewProfile and setting arrays
              (bind _returnvalue (`|SpawnActorFromClass` "/Game/MainMenu/Entities/BP_PlayerProfile.BP_PlayerProfile_C" (`self.Spawn Transform`) "AdjustIfPossibleButAlwaysSpawn" "OverrideRootScale" null null))
              (bind _output_get (set `self.LastCreatedPlayerProfile` _returnvalue))
              (set `/Game/MainMenu/Entities/BP_PlayerProfile.ProfileName` (`/Game/MainMenu/CreateProfileMenu/UI_CreateNewProfileMenu.CurrentProfileName` (`self.CreateNewProfileMenuReference`)) _output_get)
              (bind _returnvalue_2 (`KismetArrayLibrary.Array_Add` _localarrayofplayerprofiles _lastcreatedplayerprofile))
              (set `/Game/MainMenu/Entities/BP_PlayerProfile.profileId` _returnvalue_2 _lastcreatedplayerprofile)
              (set `/Game/MainMenu/BP_GameInstance.ArrayOfPlayerProfile` _localarrayofplayerprofiles (`self.GameInstanceReference`))
              (`Widget.RemoveFromParent` (`self.CreateNewProfileMenuReference`))
              (`KismetSystemLibrary.CollectGarbage`))))))))

(fn `UserConstructionScript`)